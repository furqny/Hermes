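; BP_Dummy is a target dummy for the InteractiveInventory showcase that moves into place when a Character approaches and retreats when damaged.
; A one-shot overlap box enables Tick-driven interpolation of the mesh's location and rotation toward the DummyEnd transform.
; Any damage sets Hit, which sends the mesh back to its starting transform at double speed and plays a hit sound with randomized volume and pitch.
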(event `self.ReceiveBeginPlay`
  (set `self.StartTransform` (`SceneComponent.GetRelativeTransform` (`self.DummyMesh`))))

(event `MoveDummy`
  (set `self.StartMoveDummy` true))

(event `self.ReceiveTick`
  (params (DeltaSeconds :type "Float (single-precision)"))
  (bind _hit (`self.Hit`))
  (bind _starttransform_location (`KismetMathLibrary.BreakTransform` (`self.StartTransform`)))
  (bind (_starttransform_location_2 _starttransform_rotation) (`KismetMathLibrary.BreakTransform` (`self.StartTransform`)))
  (bind _dummyinterpspeed (`self.DummyInterpSpeed`))
  (bind _returnvalue (`KismetMathLibrary.SelectFloat` (* _dummyinterpspeed 2.0) _dummyinterpspeed _hit))
  (if (`self.StartMoveDummy`)
    (`SceneComponent.K2_SetRelativeLocationAndRotation` (`self.DummyMesh`) (`KismetMathLibrary.VInterpTo` (`SceneComponent.RelativeLocation` (`self.DummyMesh`)) (`KismetMathLibrary.SelectVector` _starttransform_location (`SceneComponent.RelativeLocation` (`self.DummyEnd`)) _hit) DeltaSeconds _returnvalue) (`KismetMathLibrary.RInterpTo` (`SceneComponent.RelativeRotation` (`self.DummyMesh`)) (`KismetMathLibrary.SelectRotator` _starttransform_rotation (`SceneComponent.RelativeRotation` (`self.DummyEnd`)) (`self.Hit`)) DeltaSeconds _returnvalue) false false)))

(event `self.OverlapBox.OnComponentBeginOverlap`
  (params (OverlappedComponent :type "PrimitiveComponent Object Reference") (OtherActor :type "Actor Object Reference") (OtherComp :type "PrimitiveComponent Object Reference") (OtherBodyIndex :type Integer) (bFromSweep :type Boolean) (SweepResult :type "HitResult Structure (by ref)"))
  (cast `Character` OtherActor)
  (`self.MoveDummy`)
  (`PrimitiveComponent.SetCollisionEnabled` (`self.OverlapBox`) "NoCollision"))

(event `self.ReceiveAnyDamage`
  (params (Damage :type "Float (single-precision)") (DamageType :type "DamageType Object Reference") (InstigatedBy :type "Controller Object Reference") (DamageCauser :type "Actor Object Reference"))
  (set `self.Hit` true)
  (`GameplayStatics.PlaySoundAtLocation` "/Game/InteractiveInventory/Audio/SoundCue/SC_DummyHit.SC_DummyHit" (`SceneComponent.K2_GetComponentLocation` (`self.DummyEnd`)) (struct) (`KismetMathLibrary.RandomFloatInRange` 0.7 0.9) (`KismetMathLibrary.RandomFloatInRange` 0.9 1.0) 0.0 null null null null))

(fn `UserConstructionScript`)