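; Base interactable actor for the interactive inventory, with an interact box, a key-prompt widget and a placeholder InteractReceived event for overriding.
; Enabling or disabling routes through server and multicast events, telling overlapping actors' BPC_interact components to begin or end overlap.
; The prompt circle shows only while interactable, and a timer hides the widget afterward for performance.
; Helpers compute acceptable range from box extent and toggle target meshes, equipped items and interaction together.
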(event `self.ReceiveBeginPlay`
  ;[1 0.9925 0.7427] Begin Play
  (bind _aswbp_e_widget (cast `/Game/InteractiveInventory/Blueprints/UI/HUD/WBP_E_Widget` (`WidgetComponent.GetWidget` (`self.Widget`))))
  (set `self.OwnInteractionWidget` _aswbp_e_widget))

(event `Server_EnableInteraction`
  (params (Enable :type Boolean))
  ;[1 1 1] Comment
  (`self.Multicast_EnableInteract` Enable))

(event `InteractReceived`
  (params (NewOwner :type "Actor Object Reference"))
  ;[1 1 1] Interaction called by an other actor
  (`KismetSystemLibrary.PrintString` "override interact"))

(event `Multicast_EnableInteract`
  (params (Enable :type Boolean))
  ;[1 1 1] Hide or show items for the players
  (if Enable
    (set `self.bInteractable` true)
    (for _array_element (`self.GetOverlappingActors` null)
      (bind _returnvalue (`self.HasValidInteractClass` _array_element)
        (:`Is Valid`
          (`/Game/InteractiveInventory/Blueprints/Interact/BPC_interact.SafeOverlapBegin` _returnvalue self))))
    (else
      (for _array_element_2 (`self.GetOverlappingActors` null)
        (bind _returnvalue_2 (`self.HasValidInteractClass` _array_element_2)
          (:`Is Valid`
            (`/Game/InteractiveInventory/Blueprints/Interact/BPC_interact.SafeOverlapEnd` _returnvalue_2 self))))
      (`/Engine/EditorBlueprintResources/ActorMacros.Switch Has Authority`
        (:`Authority`
          (set `self.bInteractable` false))))))

(fn `EnableInteraction`
  (params (bEnable :type Boolean))
  ;[1 1 1] Enable/Disable Interaction
  (`self.Server_EnableInteraction` bEnable))

(fn `GetCanReceiveInteract`
  (returns (ReturnValue :type Boolean))
  ;[1 1 1] Get Is Interactable
  (return (`self.bInteractable`)))

(fn `GetMinAcceptableRange`
  (returns (MinDistance :type "Float (double-precision)"))
  ;[1 1 1] If
  (return (+ (* (`KismetMathLibrary.VSizeXY` (`BoxComponent.GetScaledBoxExtent` (`self.InteractBox`))) (`self.MInAcceptableRangeMultiplier`)) (`self.MInAcceptableRangeExtender`))))

(fn `HideWidget`
  ;[1 1 1] After a period of time Auto HideWidget
  (`SceneComponent.SetVisibility` (`self.Widget`) false false))

(fn `ShowActorWithAttachmentsLocal`
  (params (Target :type "Actor Object Reference") (NewVisibility :type Boolean))
  (locals (InventoryRef :type "/Game/InteractiveInventory/Blueprints/Inventory/BPC_Inventory Object Reference") (SceneComponentsRef :type "Array of SceneComponent Object Reference"))
  (`|ExecutionSequence`
    (:`then_0`
      (bind _output_get (set `local.SceneComponentsRef` (`self.K2_GetComponentsByClass` Target "/Script/Engine.SkeletalMeshComponent")))
      (if (`KismetArrayLibrary.Array_IsNotEmpty` _output_get)
        (for _array_element (`local.SceneComponentsRef`)
          (`SceneComponent.SetVisibility` _array_element (`local.NewVisibility`) false))))
    (:`then_1`
      (bind _output_get_2 (set `local.SceneComponentsRef` (`self.K2_GetComponentsByClass` Target "/Script/Engine.StaticMeshComponent")))
      (if (`KismetArrayLibrary.Array_IsNotEmpty` _output_get_2)
        (for _array_element_2 (`local.SceneComponentsRef`)
          (`SceneComponent.SetVisibility` _array_element_2 (`local.NewVisibility`) false))))
    (:`then_2`
      (bind _output_get_3 (set `local.InventoryRef` (`self.GetComponentByClass` Target "/Game/InteractiveInventory/Blueprints/Inventory/BPC_Inventory.BPC_Inventory_C")))
      (`/Engine/EditorBlueprintResources/StandardMacros.IsValid` _output_get_3
        (:`Is Valid`
          (`/Game/InteractiveInventory/Blueprints/Inventory/BPC_Inventory.HideEquippedActorsLocal` (`local.InventoryRef`) (`local.NewVisibility`)))))
    (:`then_3`
      (`self.EnableInteraction` (`local.NewVisibility`)))))

(fn `ShowCircle`
  (params (Show :type Boolean))
  (returns (Done :type Boolean))
  (bind _owninteractionwidget (`self.OwnInteractionWidget`))
  ;[1 1 1] Show/Hide press Cricle animation on widget
  ; Then disable it for better performance
  (if (`self.bInteractable`)
    (`/Engine/EditorBlueprintResources/StandardMacros.IsValid` (`self.OwnInteractionWidget`)
      (:`Is Valid`
        (if Show
          (`/Game/InteractiveInventory/Blueprints/UI/HUD/WBP_E_Widget.show_Interaction_Circle` _owninteractionwidget true)
          (`KismetSystemLibrary.K2_ClearAndInvalidateTimerHandle` (`self.AutoHideWidgetTimerRef`))
          (`SceneComponent.SetVisibility` (`self.Widget`) true false)
          (return true)
          (else
            (`/Game/InteractiveInventory/Blueprints/UI/HUD/WBP_E_Widget.show_Interaction_Circle` _owninteractionwidget false)
            (bind _returnvalue (`KismetSystemLibrary.K2_SetTimer` null "HideWidget" 1.0))
            (set `self.AutoHideWidgetTimerRef` _returnvalue)
            (return true))))
      (:`Is Not Valid`
        (return false)))
    (else
      (return false))))

(fn `ShowKey`
  (params (Show :type Boolean))
  ;[1 1 1] Show/Hide press key animation on widget
  (`/Engine/EditorBlueprintResources/StandardMacros.IsValid` (`self.OwnInteractionWidget`)
    (:`Is Valid`
      (`/Game/InteractiveInventory/Blueprints/UI/HUD/WBP_E_Widget.Show_Key` (`self.OwnInteractionWidget`) Show))))

(fn `UserConstructionScript`)