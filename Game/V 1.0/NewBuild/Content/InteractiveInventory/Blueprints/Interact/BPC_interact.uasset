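; Character component that lets the local player detect and interact with nearby BP_Interactable actors.
; Sphere overlaps, gated by a replicated CanDoInteract flag updated on controller changes, show circles and fill a candidate list that enables Tick.
; Tick picks a target by camera sphere trace or closest distance, showing its key within range, using a height-tolerant distance check.
; Interaction goes through a server event to the target's InteractReceived.
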(event `OnCharacterControllerChanged`
  (params (Pawn :type "Pawn Object Reference") (OldController :type "Controller Object Reference") (NewController :type "Controller Object Reference"))
  ;[1 1 1] Comment
  (if (and (`KismetSystemLibrary.IsValid` OldController) (== OldController (`self.PlayerControllerRef`)))
    (`self.EnableCanDoInteraction` false)
    (else
      (bind _asplayer_controller (cast `PlayerController` (`Pawn.GetController` (`self.CharacterRef`))))
      (bind _output_get (set `self.PlayerControllerRef` _asplayer_controller))
      (set `self.bIsLocalPlayerController` (`Controller.IsLocalController` _output_get))
      (`self.EnableCanDoInteraction` true))))

(event `self.ReceiveBeginPlay`
  ;[1 1 1] 0-Get the references for the players(Which has a valid local player controller)
  ; 1-Get the interact collision Ref
  ; 2-Bind the interaction for players
  (`|ExecutionSequence`
    (:`then_0`
      (bind _ascharacter (cast `Character` (`self.GetOwner`)))
      (bind _output_get (set `self.CharacterRef` _ascharacter))
      (add `Pawn.ReceiveControllerChangedDelegate` _output_get (`|CreateDelegate` :!event `OnCharacterControllerChanged`))
      (`self.OnCharacterControllerChanged` null))
    (:`then_1`
      (set `self.InteractCollision` (`Actor.GetComponentByClass` (`self.GetOwner`) "/Script/Engine.SphereComponent"))
      (set `self.CapsuleComponent` (`Actor.GetComponentByClass` (`self.GetOwner`) "/Script/Engine.CapsuleComponent")))
    (:`then_2`
      (if (`self.bIsLocalPlayerController`)
        (set `self.CameraRef` (`PlayerController.PlayerCameraManager` (`self.PlayerControllerRef`)))
        (`self.SetComponentTickEnabled` true)
        (`|ExecutionSequence`
          (:`then_0`
            (`/Engine/EditorBlueprintResources/StandardMacros.IsValid` (`self.InteractCollision`)
              (:`Is Valid`
                (add `PrimitiveComponent.OnComponentBeginOverlap` (`self.InteractCollision`) (`|CreateDelegate` :!event `OnComponentBeginOverlap`))
                (add `PrimitiveComponent.OnComponentEndOverlap` (`self.InteractCollision`) (`|CreateDelegate` :!event `OnComponentEndOverlap`))))))))))

(event `OnComponentEndOverlap`
  (params (OverlappedComponent :type "PrimitiveComponent Object Reference") (OtherActor :type "Actor Object Reference") (OtherComp :type "PrimitiveComponent Object Reference") (OtherBodyIndex :type Integer))
  ;[1 1 1] OnOverlapEnd
  (`self.OverlapEnd` OtherActor))

(event `Server_interact`
  (params (Target :type "/Game/InteractiveInventory/Blueprints/Interact/BP_Interactable Object Reference"))
  ;[1 1 1] Request interact On server
  (`/Game/InteractiveInventory/Blueprints/Interact/BP_Interactable.InteractReceived` Target (`self.GetOwner`)))

(event `OnComponentBeginOverlap`
  (params (OverlappedComponent :type "PrimitiveComponent Object Reference") (OtherActor :type "Actor Object Reference") (OtherComp :type "PrimitiveComponent Object Reference") (OtherBodyIndex :type Integer) (bFromSweep :type Boolean) (SweepResult :type "HitResult Structure (by ref)"))
  ;[1 1 1] OnOverlapBegin
  (`self.OverlapBegin` OtherActor))

(event `self.ReceiveTick`
  (params (DeltaSeconds :type "Float (single-precision)"))
  ;[1 1 1] Depends on bNeedVisualTrace variable, try to find the main target
  (if (`self.bNeedVisualTrace`)
    (`self.LineTraceForInteract`)
    (else
      (bind _closestactor (`self.GetClosestActorInList`))
      (`self.OnNewActorDetected` _closestactor))))

(fn `AddObject`
  (params (NewAddedObject :type "/Game/InteractiveInventory/Blueprints/Interact/BP_Interactable Object Reference"))
  ;[1 1 1] Add a new object To the list
  (if (`self.bIsLocalPlayerController`)
    (`KismetArrayLibrary.Array_Add` (`self.ActorsList`) NewAddedObject)
    (`self.SetComponentTickEnabled` true)))

(fn `CustomDistanceTo`
  (params (OtherActor :type "Actor Object Reference"))
  (returns (ReturnValue :type "Float (double-precision)"))
  (bind (_returnvalue_x _returnvalue_y _returnvalue_z) (`KismetMathLibrary.BreakVector` (- (`Actor.K2_GetActorLocation` OtherActor) (`Actor.K2_GetActorLocation` (`self.GetOwner`)))))
  (bind _returnvalue (- (`KismetMathLibrary.Abs` _returnvalue_z) 90.0))
  ;[1 1 1] character has a height about 180cm
  ; for z axis, about 90 cm of z distance is ignored
  (return (`KismetMathLibrary.VSize` (`KismetMathLibrary.MakeVector` _returnvalue_x _returnvalue_y (select `bool` (> _returnvalue 0.0) :`true` _returnvalue)))))

(fn `DeleteCurrentWidget`
  ;[1 1 1] Delete Last If Available
  (bind _current_bp_interactable (`self.Current_BP_Interactable`)
    (:`then`
      (`/Game/InteractiveInventory/Blueprints/Interact/BP_Interactable.ShowKey` _current_bp_interactable false)
      (set `self.Current_BP_Interactable` null))
    (:`else`)))

(fn `EnableCanDoInteraction`
  (params (bCanDoInteract :type Boolean))
  ;[1 1 1] Comment
  (set `self.bCanDoInteract` bCanDoInteract))

(fn `GetCanDoInteract`
  (returns (bCanDoInteract :type Boolean))
  ;[1 1 1] Returns Can Do interact
  (return (`self.bCanDoInteract`)))

(fn `GetClosestActorInList`
  (returns (ClosestActor :type "Actor Object Reference"))
  (locals (MinDistanceFound :type "Float (double-precision)" :default 9999.0) (MinDistanceActor :type "Actor Object Reference") (CurrentTesedActor :type "Actor Object Reference") (CurrentDistance :type "Float (single-precision)" :default 0.0))
  ;[1 1 1] Search in Array for closest InteractableActor
  (for _array_element (`self.ActorsList`)
    (set `local.CurrentTesedActor` _array_element)
    (set `local.CurrentDistance` (`Actor.GetDistanceTo` (`self.CharacterRef`) (`local.CurrentTesedActor`)))
    (if (< (`local.CurrentDistance`) (`local.MinDistanceFound`))
      (set `local.MinDistanceActor` (`local.CurrentTesedActor`))
      (set `local.MinDistanceFound` (`local.CurrentDistance`))))
  (return (`local.MinDistanceActor`)))

(fn `getIsLocalPlayer`
  (returns (bIsLocalPlayerController :type Boolean))
  (return (`self.bIsLocalPlayerController`)))

(fn `InteractWithCurrentValidActor`
  ;[1 1 1] Try to interact
  (bind _current_bp_interactable (`self.Current_BP_Interactable`)
    (:`then`
      (`self.Server_interact` _current_bp_interactable))
    (:`else`)))

(fn `LineTraceForInteract`
  ;[1 1 1] Trace a sphere from camera toward forward to find any actor that are in sight
  (bind _cameraref (`self.CameraRef`)
    (:`then`
      (bind _returnvalue (`PlayerCameraManager.GetCameraLocation` _cameraref))
      (bind _outhit (`KismetSystemLibrary.SphereTraceSingle` :`Start` _returnvalue :`End` (+ _returnvalue (* (`KismetMathLibrary.GetForwardVector` (`PlayerCameraManager.GetCameraRotation` _cameraref)) 2000.0)) :`Radius` 45.0 :`TraceChannel` "TraceTypeQuery3" :`DrawTime` 0.1))
      (`self.OnNewActorDetected` (`.HitActor` (`GameplayStatics.BreakHitResult` _outhit))))
    (:`else`)))

(fn `OnNewActorDetected`
  (params (CurrentHitActor :type "Actor Object Reference"))
  (locals (LocalHitActor :type "Actor Object Reference"))
  (bind _output_get (set `local.LocalHitActor` CurrentHitActor))
  (`/Engine/EditorBlueprintResources/StandardMacros.IsValid` _output_get
    (:`Is Valid`
      (if (!= (`local.LocalHitActor`) (`self.Current_BP_Interactable`))
        (bind _asbp_interactable (cast `/Game/InteractiveInventory/Blueprints/Interact/BP_Interactable` (`local.LocalHitActor`)))
        (bind _output_get_2 (set `self.LastActorAcceptableDistance` (`/Game/InteractiveInventory/Blueprints/Interact/BP_Interactable.GetMinAcceptableRange` _asbp_interactable)))
        (if (< (`self.CustomDistanceTo` (`local.LocalHitActor`)) _output_get_2)
          (`self.DeleteCurrentWidget`)
          (bind _output_get_3 (set `self.Current_BP_Interactable` _asbp_interactable))
          (`/Game/InteractiveInventory/Blueprints/Interact/BP_Interactable.ShowKey` _output_get_3 true)
          (else
            (`self.DeleteCurrentWidget` :!label _label)))
        (elif (not (< (`self.CustomDistanceTo` (`local.LocalHitActor`)) (`self.LastActorAcceptableDistance`)))
          (`/Game/InteractiveInventory/Blueprints/Interact/BP_Interactable.ShowKey` (`self.Current_BP_Interactable`) false)
          (set `self.Current_BP_Interactable` null))))
    (:`Is Not Valid`
      (goto _label))))

(fn `OnRep_bCanDoInteract`
  ;[1 1 1] Enable/Disable Interaction On owner
  (if (`self.bIsLocalPlayerController`)
    (if (`self.bCanDoInteract`)
      (for _array_element (`Actor.GetOverlappingActors` (`self.CharacterRef`) "/Game/InteractiveInventory/Blueprints/Interact/BP_Interactable.BP_Interactable_C")
        (`self.OverlapBegin` _array_element))
      (else
        (for _array_element_2 (`Actor.GetOverlappingActors` (`self.CharacterRef`) "/Game/InteractiveInventory/Blueprints/Interact/BP_Interactable.BP_Interactable_C")
          (`self.OverlapEnd` _array_element_2))))))

(fn `OverlapBegin`
  (params (InputActor :type "Actor Object Reference"))
  ;[1 1 1] On overlap begin
  (if (`self.bCanDoInteract`)
    (`self.InvalidOwningChildActor` InputActor
      (:`Valid`
        (bind _asbp_interactable (cast `/Game/InteractiveInventory/Blueprints/Interact/BP_Interactable` InputActor))
        (bind _done (`/Game/InteractiveInventory/Blueprints/Interact/BP_Interactable.ShowCircle` _asbp_interactable true))
        (if _done
          (`self.AddObject` _asbp_interactable))))))

(fn `OverlapEnd`
  (params (InputActor :type "Actor Object Reference"))
  ;[1 1 1] On overlap End
  (`self.InvalidOwningChildActor` InputActor
    (:`Valid`
      (bind _asbp_interactable (cast `/Game/InteractiveInventory/Blueprints/Interact/BP_Interactable` InputActor))
      (`/Game/InteractiveInventory/Blueprints/Interact/BP_Interactable.ShowCircle` _asbp_interactable false)
      (`self.RemoveObject` _asbp_interactable))))

(fn `RemoveObject`
  (params (ObjectToRemove :type "/Game/InteractiveInventory/Blueprints/Interact/BP_Interactable Object Reference"))
  ;[1 1 1] Remove object From Interaction list
  (if (`self.bIsLocalPlayerController`)
    (`KismetArrayLibrary.Array_RemoveItem` (`self.ActorsList`) ObjectToRemove)
    (if (`KismetArrayLibrary.Array_IsEmpty` (`self.ActorsList`))
      (`self.SetComponentTickEnabled` false)
      (`self.DeleteCurrentWidget`))))

(fn `SafeOverlapBegin`
  (params (InputActor :type "Actor Object Reference"))
  (if (`self.getIsLocalPlayer`)
    (`self.OverlapBegin` InputActor)))

(fn `SafeOverlapEnd`
  (params (InputActor :type "Actor Object Reference"))
  (if (`self.getIsLocalPlayer`)
    (`self.OverlapEnd` InputActor)))

(fn `SetOwnBPInteractable`
  (params (Own_BPInteractable :type "Actor Object Reference"))
  (bind _output_get (set `self.Own_BPInteractable` Own_BPInteractable))
  (bind _asbp_interactable (cast `/Game/InteractiveInventory/Blueprints/Interact/BP_Interactable` _output_get))
  (`self.RemoveObject` _asbp_interactable))