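; BP_Projectile is the weapon projectile actor, which damages what it hits and destroys itself on impact or after a short lifetime.
; Construction applies Speed to the movement component, and BeginPlay sets the VFX asset and binds the hit event.
; On hit, positive damage is applied with authority through BPI_CustomDamage, falling back to standard ApplyDamage.
; It also passes damaging hits to its owning BP_Weapon for impact visuals.
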(event `self.ReceiveBeginPlay`
  ;[1 1 1] Set Material in begin play
  (`NiagaraComponent.SetAsset` (`self.ProjectileVFXComponent`) (`self.In Asset`) true)
  (`|ExecutionSequence`
    (:`then_0`
      (add `self.OnActorHit` (`|CreateDelegate` :!event `HitEvent`)))
    (:`then_1`
      (`KismetSystemLibrary.Delay` 2.0)
      (`self.K2_DestroyActor`))))

(event `HitEvent` :!signature `self.OnActorHit`
  (params (SelfActor :type "Actor Object Reference") (OtherActor :type "Actor Object Reference") (NormalImpulse :type "Vector Structure") (Hit :type "HitResult Structure (by ref)"))
  (set `self.HitActor` OtherActor)
  (set `self.Hit` Hit)
  (`|ExecutionSequence`
    (:`then_0`
      ;[1 1 1] ApplyDamage
      (if (and (> (`self.Damage`) 0.0) (`self.HasAuthority`))
        (if (`KismetSystemLibrary.DoesImplementInterface` (`self.HitActor`) "/Game/InteractiveInventory/Blueprints/Interfaces/BPI_CustomDamage.BPI_CustomDamage_C")
          (message `/Game/InteractiveInventory/Blueprints/Interfaces/BPI_CustomDamage.CustomApplyDamage` (`self.HitActor`) (`self.Damage`) (`self.Hit`) (`self.GetInstigator`) (`self.Weapon`))
          (else
            (`GameplayStatics.ApplyDamage` (`self.HitActor`) (`self.Damage`) (`self.GetInstigatorController` (`self.GetInstigator`)) (`self.GetInstigator`))))))
    (:`then_1`
      ;[1 1 1] hit visual
      (if (> (`self.Damage`) 0.0)
        (bind _asbp_weapon (cast `/Game/InteractiveInventory/Blueprints/Weapon/BP_Weapon` (`self.GetOwner`)))
        (`/Game/InteractiveInventory/Blueprints/Weapon/BP_Weapon.OnProjectileHit` _asbp_weapon (`self.Hit`))))
    (:`then_2`
      ;[1 1 1] Comment
      (`self.K2_DestroyActor`))))

(fn `UserConstructionScript`
  (bind _projectilevfxmovementcomp (`self.ProjectileVFXMovementComp`))
  (bind _output_get (set `ProjectileMovementComponent.InitialSpeed` (`self.Speed`) _projectilevfxmovementcomp))
  (set `ProjectileMovementComponent.MaxSpeed` _output_get _projectilevfxmovementcomp))