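; Blueprint function library of helpers for the inventory map system, mostly for looking up map sections in DT_SectionsData.
; Row order serves as the section number, with functions converting between row name and index.
; Section data is fetched by row name, falling back to a zero-width struct when the row is missing.
; A separate math helper clamps a value symmetrically between negative and positive limits.
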(fn `ClampFloatMirror`
  (params (Value :type "Float (double-precision)") (AbsMax :type "Float (double-precision)"))
  (returns (ReturnValue :type "Float (double-precision)"))
  ;[1 1 1] Clamp data between -absmax<your value < +absmax
  (return (`KismetMathLibrary.FClamp` Value (* AbsMax -1.0) AbsMax)))

(fn `GetSectionData`
  (params (RowName :type Name))
  (returns (`Out Row` :type "/Game/InteractiveInventory/Structure/F_SectionData Structure"))
  ;[1 1 1] Get section data
  (bind _returnvalue (`|GetDataTableRow` "/Game/InteractiveInventory/Blueprints/Map/DT_SectionsData.DT_SectionsData" RowName)
    (:`then`
      (return _returnvalue))
    (:`RowNotFound`
      (return (make `/Game/InteractiveInventory/Structure/F_SectionData` null)))))

(fn `GetSectionName`
  (params (SectionNumber :type "Float (double-precision)"))
  (returns (SectionName :type Name))
  (locals (Number :type Integer :default 0))
  (bind _output_get (set `local.Number` (`KismetMathLibrary.FTrunc` SectionNumber)))
  (bind _outrownames (`DataTableFunctionLibrary.GetDataTableRowNames` "/Game/InteractiveInventory/Blueprints/Map/DT_SectionsData.DT_SectionsData"))
  (if (`KismetArrayLibrary.Array_IsValidIndex` _outrownames (`local.Number`))
    (return (`|GetArrayItem` _outrownames _output_get))))

(fn `GetSectionNumber`
  (params (RowName :type Name))
  (returns (SectionNumber :type "Float (double-precision)"))
  (locals (FoundedSection :type "Float (double-precision)" :default 0.0))
  ;[1 1 1] Get section number in list
  (bind _outrownames (`DataTableFunctionLibrary.GetDataTableRowNames` "/Game/InteractiveInventory/Blueprints/Map/DT_SectionsData.DT_SectionsData"))
  (for (_array_element _array_index) _outrownames
    (if (== _array_element RowName)
      (set `local.FoundedSection` (`KismetMathLibrary.Conv_IntToDouble` _array_index))
      (break)))
  (return (`local.FoundedSection`)))