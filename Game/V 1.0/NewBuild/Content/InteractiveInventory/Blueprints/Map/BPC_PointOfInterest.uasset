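; Actor component that marks its owner as a point of interest, shown as an icon on the inventory map.
; On BeginPlay it tags the owner and takes floor and section from an overlapping BP_Room (markers excepted), also notifying the room of pawn owners.
; Floor changes or activation recreate the icon through the last WBP_Map widget found.
; Helpers supply optional actor-yaw rotation and a switchable image from an icon array.
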(event `GetRoomData`
  (bind _returnvalue (`self.GetOwner`))
  (bind _overlappingactors (`Actor.GetOverlappingActors` _returnvalue "/Game/InteractiveInventory/Blueprints/Map/BP_Room.BP_Room_C"))
  ;[1 1 1] Check if there is any room around it and get the room data
  (`KismetSystemLibrary.Delay` 0.1)
  (cast `/Game/InteractiveInventory/Blueprints/Map/BP_Marker` _returnvalue
    (:`CastFailed`
      (if (`KismetArrayLibrary.Array_IsNotEmpty` _overlappingactors)
        (bind _asbp_room (cast `/Game/InteractiveInventory/Blueprints/Map/BP_Room` (`|GetArrayItem` _overlappingactors)))
        (bind (_floor _section) (`/Game/InteractiveInventory/Blueprints/Map/BP_Room.GetFloorAndSection` _asbp_room))
        (`self.SetFloorAndSection` _floor _section)))))

(event `self.ReceiveBeginPlay`
  (bind _overlappingactors (`Actor.GetOverlappingActors` (`self.GetOwner`) "/Game/InteractiveInventory/Blueprints/Map/BP_Room.BP_Room_C"))
  (`|ExecutionSequence`
    (:`then_0`
      (`KismetArrayLibrary.Array_AddUnique` (`Actor.Tags` (`self.GetOwner`)) "Map_PointOfInterest"))
    (:`then_1`
      (`self.GetRoomData`)
      (bind _ascharacter (cast `Character` (`self.GetOwner`)))
      (set `self.CharacterRef` _ascharacter))
    (:`then_2`
      (if (`KismetArrayLibrary.Array_IsNotEmpty` _overlappingactors)
        (bind _asbp_room (cast `/Game/InteractiveInventory/Blueprints/Map/BP_Room` (`|GetArrayItem` _overlappingactors)))
        (bind _aspawn (cast `Pawn` (`self.GetOwner`)))
        (`/Game/InteractiveInventory/Blueprints/Map/BP_Room.OnCharacterOverlapped` _asbp_room _aspawn)))))

(fn `AddIconToMap`
  ;[1 1 1] Get last created map widget and update data
  (`self.RemoveIcon`)
  (bind _foundwidgets (`WidgetBlueprintLibrary.GetAllWidgetsOfClass` "/Game/InteractiveInventory/Blueprints/UI/Map/WBP_Map.WBP_Map_C" false))
  (if (`KismetArrayLibrary.Array_IsNotEmpty` _foundwidgets)
    (bind _iconwidget (`/Game/InteractiveInventory/Blueprints/UI/Map/WBP_Map.CreateIconWidget` (`|GetArrayItem` _foundwidgets (`KismetArrayLibrary.Array_LastIndex` _foundwidgets)) (`self.GetOwner`)))
    (set `self.Icon WidgetRef` _iconwidget)))

(fn `ChangeSelectedNumber`
  (params (SelectedImageNumber :type Integer))
  (bind _icon_widgetref (`self.Icon WidgetRef`))
  ;[1 1 1] Change image of the bpc in map
  (bind _output_get (set `self.SelectedImageNumber` SelectedImageNumber))
  (`/Engine/EditorBlueprintResources/StandardMacros.IsValid` _icon_widgetref
    (:`Is Valid`
      (`/Game/InteractiveInventory/Blueprints/UI/Map/WBP_POI.UpdateImage` _icon_widgetref (`|GetArrayItem` (`self.IconImage`) _output_get)))))

(fn `GetDisplayRotation`
  (returns (ReturnValue :type "Float (single-precision)"))
  (bind (_returnvalue_roll _returnvalue_pitch _returnvalue_yaw) (`KismetMathLibrary.BreakRotator` (`Actor.K2_GetActorRotation` (`self.GetOwner`))))
  ;[1 1 1] Get display rotation
  (return (select `bool` (`self.bShouldRotateWithActor`) :`true` (+ _returnvalue_yaw 90.0) :!type "Float (single-precision)")))

(fn `GetImageToDisplay`
  (returns (Output :type "Texture2D Object Reference"))
  ;[1 1 1] get which image to display from "IconImage" array
  (return (`|GetArrayItem` (`self.IconImage`) (`self.SelectedImageNumber`))))

(fn `GetIsActive`
  (returns (bActive :type Boolean))
  (return (`self.bActive`)))

(fn `RemoveIcon`
  (bind _icon_widgetref (`self.Icon WidgetRef`))
  (`/Engine/EditorBlueprintResources/StandardMacros.IsValid` _icon_widgetref
    (:`Is Valid`
      (`Widget.RemoveFromParent` _icon_widgetref))))

(fn `SetFloorAndSection`
  (params (Floor :type "Float (double-precision)") (InSection :type Name))
  ;[1 1 1] On floor and section changed, try to update map if map is open
  (set `self.Floor` Floor)
  (set `self.Section` InSection)
  (`self.AddIconToMap`))

(fn `SetIsActive`
  (params (InActive :type Boolean))
  ;[1 1 1] Comment
  (if (xor InActive (`self.bActive`))
    (bind _output_get (set `self.bActive` (`local.InActive`)))
    (if _output_get
      (`self.AddIconToMap`))))