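; Actor component that lets a player place and remove a single map landmark marker, with spawn and destroy sounds.
; Requesting a landmark near the current one in 2D removes it; elsewhere, it replaces it.
; New markers take their Section and Floor from the Map_Data parameter collection.
; Server events spawn and destroy the BP_Marker actor, keeping only the last reference.
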(event `Server_CreateLandmark`
  (params (`Spawn Transform Location` :type "Vector Structure") (Section :type Name) (Floor :type "Float (double-precision)"))
  (`self.DeleteLandmarkOnServer`)
  (bind _returnvalue (`|SpawnActorFromClass` "/Game/InteractiveInventory/Blueprints/Map/BP_Marker.BP_Marker_C" (`KismetMathLibrary.MakeTransform` `Spawn Transform Location`) "Undefined" "MultiplyWithRoot" null Section Floor null))
  (set `self.LastLandmarkRef` _returnvalue))

(event `Server_DeleteMarker`
  (`self.DeleteLandmarkOnServer`))

(fn `Create Landmark`
  (params (`Spawn Transform Location` :type "Vector Structure"))
  (`self.LastLandmarkRef`
    (:`then`
      (if (== (`KismetMathLibrary.Conv_VectorToVector2D` (`Actor.K2_GetActorLocation` (`self.LastLandmarkRef`))) (`KismetMathLibrary.Conv_VectorToVector2D` (`local.Spawn Transform Location`)) :`ErrorTolerance` 20.0)
        (`self.Server_DeleteMarker`)
        (`GameplayStatics.PlaySound2D` (`self.MarkerDestroySound`) 1.0 1.0 0.0 null null)
        (else
          (`self.Server_DeleteMarker`)
          (bind _returnvalue (`KismetMaterialLibrary.GetScalarParameterValue` "/Game/InteractiveInventory/Blueprints/Map/Map_Data.Map_Data" "Section" :!label _label))
          (bind _returnvalue_2 (`KismetMaterialLibrary.GetScalarParameterValue` "/Game/InteractiveInventory/Blueprints/Map/Map_Data.Map_Data" "Floor"))
          (`self.Server_CreateLandmark` (`local.Spawn Transform Location`) (`/Game/InteractiveInventory/Blueprints/Map/MapFunctionLibrary.GetSectionName` _returnvalue) _returnvalue_2)
          (`GameplayStatics.PlaySound2D` (`self.MarkerSpawnSound`) 1.0 1.0 0.0 null null))))
    (:`else`
      (goto _label))))

(fn `DeleteLandmark`
  (`self.Server_DeleteMarker`)
  (`GameplayStatics.PlaySound2D` (`self.MarkerDestroySound`) 1.0 1.0 0.0 null null))

(fn `DeleteLandmarkOnServer`
  (`/Engine/EditorBlueprintResources/StandardMacros.IsValid` (`self.LastLandmarkRef`)
    (:`Is Valid`
      (`Actor.K2_DestroyActor` (`self.LastLandmarkRef`)))))