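; Room actor for the inventory map that tracks the player's location and whether the room is unseen, has items or is fully searched.
; When a pawn enters its box, it copies floor and section to that pawn's point-of-interest component.
; For locally controlled pawns, it also sets search status and writes location to the Map_Data material parameter collection.
; Mask color queries re-check overlapping "Collectable"-tagged actors and return status as a number.
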(event `self.Box.OnComponentBeginOverlap`
  (params (OverlappedComponent :type "PrimitiveComponent Object Reference") (OtherActor :type "Actor Object Reference") (OtherComp :type "PrimitiveComponent Object Reference") (OtherBodyIndex :type Integer) (bFromSweep :type Boolean) (SweepResult :type "HitResult Structure (by ref)"))
  ;[1 1 1] On begin overlapping with player
  (bind _aspawn (cast `Pawn` OtherActor))
  (`self.OnCharacterOverlapped` _aspawn))

(fn `CopyDataToComponent`
  (params (POIComponentRef :type "/Game/InteractiveInventory/Blueprints/Map/BPC_PointOfInterest Object Reference"))
  (bind _bpc_pointofinterest (`self.BPC_PointOfInterest`))
  ;[1 1 1] Copy data to player bpc
  (`/Game/InteractiveInventory/Blueprints/Map/BPC_PointOfInterest.SetFloorAndSection` POIComponentRef (`/Game/InteractiveInventory/Blueprints/Map/BPC_PointOfInterest.Floor` _bpc_pointofinterest) (`/Game/InteractiveInventory/Blueprints/Map/BPC_PointOfInterest.Section` _bpc_pointofinterest)))

(fn `GetFloorAndSection`
  (returns (Floor :type "Float (double-precision)") (Section :type Name))
  (bind _bpc_pointofinterest (`self.BPC_PointOfInterest`))
  ;[1 1 1] Get Location data
  (return (`/Game/InteractiveInventory/Blueprints/Map/BPC_PointOfInterest.Floor` _bpc_pointofinterest) (`/Game/InteractiveInventory/Blueprints/Map/BPC_PointOfInterest.Section` _bpc_pointofinterest)))

(fn `getMaskColor`
  (returns (ReturnValue :type "Float (double-precision)"))
  ;[1 1 1] Get Color for map status
  (`self.UpdateRoomStatus`)
  (return (`KismetMathLibrary.Conv_IntToDouble` (`KismetMathLibrary.Conv_ByteToInt` (`self.MapSearchStatus`)))))

(fn `HasAnyColletable`
  (returns (HasCollectable :type Boolean))
  (locals (LocalHasCollectable :type Boolean))
  ;[1 1 1] Check if there is any collectable item in the room
  (for _array_element (`self.GetOverlappingActors` null)
    (if (`self.ActorHasTag` _array_element "Collectable")
      (set `local.LocalHasCollectable` true)
      (break)))
  (return (`local.LocalHasCollectable`)))

(fn `HasValidMask`
  (returns (ReturnValue :type Boolean))
  (return (`KismetSystemLibrary.IsValid` (`self.Mask`))))

(fn `OnCharacterOverlapped`
  (params (MapOwner :type "Pawn Object Reference"))
  (bind _returnvalue (`self.GetComponentByClass` MapOwner "/Game/InteractiveInventory/Blueprints/Map/BPC_PointOfInterest.BPC_PointOfInterest_C"))
  ;[1 1 1] On player overlaped:
  ; 1-change room color and status
  ; 2- change current room and floor
  ; 3- copy data to the player bpc
  (if (`Pawn.IsLocallyControlled` MapOwner)
    (`|ExecutionSequence`
      (:`then_0`
        (if (`|EnumEquality` (`self.MapSearchStatus`) "NewEnumerator0")
          (set `self.MapSearchStatus` (select `bool` (`self.HasAnyColletable`) :`false` "NewEnumerator2" :`true` "NewEnumerator1" :!type "/Game/InteractiveInventory/Enum/E_RoomStatus Enum"))))
      (:`then_1`
        (`KismetMaterialLibrary.SetScalarParameterValue` "/Game/InteractiveInventory/Blueprints/Map/Map_Data.Map_Data" "Floor" (`/Game/InteractiveInventory/Blueprints/Map/BPC_PointOfInterest.Floor` (`self.BPC_PointOfInterest`)))
        (`KismetMaterialLibrary.SetScalarParameterValue` "/Game/InteractiveInventory/Blueprints/Map/Map_Data.Map_Data" "Section" (`/Game/InteractiveInventory/Blueprints/Map/MapFunctionLibrary.GetSectionNumber` (`/Game/InteractiveInventory/Blueprints/Map/BPC_PointOfInterest.Section` (`self.BPC_PointOfInterest`)))))
      (:`then_2`
        (`/Engine/EditorBlueprintResources/StandardMacros.IsValid` _returnvalue :!label _label
          (:`Is Valid`
            (`self.CopyDataToComponent` _returnvalue)))))
    (else
      (goto _label))))

(fn `UpdateRoomStatus`
  ;[1 1 1] Update the map color if changes happend
  (switch `/Game/InteractiveInventory/Enum/E_RoomStatus` (`self.MapSearchStatus`)
    (:`NewEnumerator0`
      (set `self.MapSearchStatus` "NewEnumerator0"))
    (:`NewEnumerator1`
      (if (`self.HasAnyColletable`) :!label _label
        (set `self.MapSearchStatus` "NewEnumerator1")
        (else
          (set `self.MapSearchStatus` "NewEnumerator2"))))
    (:`NewEnumerator2`
      (goto _label))))

(fn `UserConstructionScript`)