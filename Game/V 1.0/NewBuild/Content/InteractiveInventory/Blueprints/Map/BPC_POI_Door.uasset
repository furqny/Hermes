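; Map point-of-interest component that represents a door on the inventory system's map.
; On BeginPlay it tags its owning actor as "Map_Door" and supplies the owner's yaw as the icon's rotation.
; Setting the door status looks up the matching image in a status-to-icon map and pushes it to the referenced icon widget, if both are valid.
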(event `self.ReceiveBeginPlay`
  (`KismetArrayLibrary.Array_AddUnique` (`Actor.Tags` (`self.GetOwner`)) "Map_Door"))

(fn `ChangeDoorImage`
  (locals (NewLocalVar :type "Texture2D Object Reference"))
  (bind _icon_widgetref (`self.Icon WidgetRef`))
  (bind _value (`BlueprintMapLibrary.Map_Find` (`self.DoorIcons`) (`self.DoorStatus`)))
  (`/Engine/EditorBlueprintResources/StandardMacros.IsValid` _value
    (:`Is Valid`
      (`/Engine/EditorBlueprintResources/StandardMacros.IsValid` _icon_widgetref
        (:`Is Valid`
          (`/Game/InteractiveInventory/Blueprints/UI/Map/WBP_Door.UpdateImage` _icon_widgetref _value))))))

(fn `GetDisplayImage`
  (returns (Image :type "Texture2D Object Reference"))
  ;[1 1 1] Get Image To display
  (return (`BlueprintMapLibrary.Map_Find` (`self.DoorIcons`) (`self.DoorStatus`))))

(fn `GetDisplayRotation`
  (returns (ReturnValue :type "Float (single-precision)"))
  (bind (_returnvalue_roll _returnvalue_pitch _returnvalue_yaw) (`KismetMathLibrary.BreakRotator` (`Actor.K2_GetActorRotation` (`self.GetOwner`))))
  ;[1 1 1] Get Door Rotation
  (return _returnvalue_yaw))

(fn `SetDoorStatus`
  (params (DoorStatus :type "/Game/InteractiveInventory/Enum/E_DoorStatus Enum" :default "NewEnumerator0"))
  (set `self.DoorStatus` DoorStatus)
  (`self.ChangeDoorImage`))