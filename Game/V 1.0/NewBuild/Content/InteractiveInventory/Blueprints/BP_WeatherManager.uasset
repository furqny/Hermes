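; BP_WeatherManager darkens the level's lighting in response to the player's karma.
; On BeginPlay it takes the first DirectionalLight in the level as the sun and binds to the main game instance's karma-changed event.
; Moderately negative karma triggers SetDarkWeather, which dims the sun and tints it deep blue, with no path to restore it.
; Both Sequence branches repeat the same check and debug print.
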(event `self.ReceiveBeginPlay`
  (bind _asbp_main_game_instance (cast `/Game/InteractiveInventory/Blueprints/GameModes-Inventory/BP_MainGameInstance` (`GameplayStatics.GetGameInstance`)))
  (bind _outactors (`GameplayStatics.GetAllActorsOfClass` "/Script/Engine.DirectionalLight"))
  (set `self.SunLight` (`|GetArrayItem` _outactors))
  (add `/Game/InteractiveInventory/Blueprints/GameModes-Inventory/BP_MainGameInstance.OnKarmaChanged` _asbp_main_game_instance (delegate `OnKarmaChanged_Event`)))

(event `OnKarmaChanged_Event`
  (params (CurrentKarma :type Integer))
  (`|ExecutionSequence`
    (:`then_0`
      (if (< CurrentKarma -1)
        (if (> CurrentKarma -11)
          (`KismetSystemLibrary.PrintString` "HOHOHOOHO" true true (struct :`R` 1.0 :`G` 0.035426 :`B` 0.846088 :`A` 1.0) 5.0)
          (`self.SetDarkWeather`))))
    (:`then_1`
      (if (< CurrentKarma -1)
        (if (> CurrentKarma -11)
          (`KismetSystemLibrary.PrintString` "HOHOHOOHO" true true (struct :`R` 1.0 :`G` 0.035426 :`B` 0.846088 :`A` 1.0) 5.0)
          (`self.SetDarkWeather`))))))

(event `SetDarkWeather`
  (bind _lightcomponent (`Light.LightComponent` (`self.SunLight`)))
  (`LightComponent.SetIntensity` _lightcomponent 0.5)
  (`LightComponent.SetLightColor` _lightcomponent (struct :`R` 0.001758 :`G` 0.059114 :`B` 0.401042 :`A` 1.0) true))

(fn `UserConstructionScript`)