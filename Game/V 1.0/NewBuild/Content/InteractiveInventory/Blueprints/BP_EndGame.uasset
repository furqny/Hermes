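; BP_EndGame is an end-of-game trigger that picks an ending from karma when the third-person character overlaps its Box.
; It reads GlobalKarmaScore from BP_MainGameInstance: below -100 prints "IYI SON" (good ending), above -99 prints "KOTU SON" (bad ending).
; Both endings share a camera fade-out, then reload the current level after a delay.
; Scores from -100 to -99 inclusive trigger neither ending.
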(event `self.Box.OnComponentHit`
  (params (HitComponent :type "PrimitiveComponent Object Reference") (OtherActor :type "Actor Object Reference") (OtherComp :type "PrimitiveComponent Object Reference") (NormalImpulse :type "Vector Structure") (Hit :type "HitResult Structure (by ref)")))

(event `self.Box.OnComponentBeginOverlap`
  (params (OverlappedComponent :type "PrimitiveComponent Object Reference") (OtherActor :type "Actor Object Reference") (OtherComp :type "PrimitiveComponent Object Reference") (OtherBodyIndex :type Integer) (bFromSweep :type Boolean) (SweepResult :type "HitResult Structure (by ref)"))
  (cast `/Game/InteractiveInventory/Blueprints/GameModes-Inventory/BP_ThirdPersonCharacter` OtherActor)
  (bind _asbp_main_game_instance (cast `/Game/InteractiveInventory/Blueprints/GameModes-Inventory/BP_MainGameInstance` (`GameplayStatics.GetGameInstance`)))
  (`|ExecutionSequence`
    (:`then_0`
      (bind _globalkarmascore (`/Game/InteractiveInventory/Blueprints/GameModes-Inventory/BP_MainGameInstance.GlobalKarmaScore` _asbp_main_game_instance))
      (if (< _globalkarmascore -100)
        (`KismetSystemLibrary.PrintString` "IYI SON")
        (`PlayerCameraManager.StartCameraFade` :`self` (`GameplayStatics.GetPlayerCameraManager` 0) :`ToAlpha` 1.0 :`Duration` 2.0 :`bHoldWhenFinished` true :!label _label)
        (`KismetSystemLibrary.Delay` 2.0)
        (bind _returnvalue (`GameplayStatics.GetCurrentLevelName` true))
        (`GameplayStatics.OpenLevel` (`KismetStringLibrary.Conv_StringToName` _returnvalue))))
    (:`then_1`
      (if (> _globalkarmascore -99)
        (`KismetSystemLibrary.PrintString` "KOTU SON")
        (goto _label)))))

(fn `UserConstructionScript`)