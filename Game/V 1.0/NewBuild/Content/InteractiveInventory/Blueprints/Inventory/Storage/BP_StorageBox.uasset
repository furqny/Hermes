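; Storage box actor that a player interacts with to open a storage UI.
; The server claims the storage manager's single active slot, takes the character as owner, multicasts the crate animation and disables interaction.
; The owning client blends the camera to the box, hides the character, then creates the HUD storage widget after a delay, pausing in standalone.
; Closing reverses these steps, releasing the active slot and owner.
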(event `self.ReceiveBeginPlay`
  (`parent.ReceiveBeginPlay`))

(event `self.InteractReceived`
  (params (NewOwner :type "Actor Object Reference"))
  ;[0.945 1 0.5841] character interacted with storage
  (bind _ascharacter (cast `Character` NewOwner))
  (`/Engine/EditorBlueprintResources/StandardMacros.IsValid` (`/Game/InteractiveInventory/Blueprints/Inventory/Storage/BP_StorageManagerActor.ActiveStorageRef` (`/Game/InteractiveInventory/Blueprints/Inventory/InventoryManagerLibrary.GetStorageManagerActorRef`))
    (:`Is Not Valid`
      (`self.StorageBegin` _ascharacter))))

(event `Client_StorageBegin`
  (params (Character :type "Character Object Reference"))
  ;[0.25 0.758 1] on clinet, continue the interact
  (set `self.CharacterRef` Character)
  (`|ExecutionSequence`
    (:`then_0`
      (bind _asbp_player_controller (cast `/Game/InteractiveInventory/Blueprints/GameModes-Inventory/BP_PlayerController` (`Pawn.GetController` (`self.CharacterRef`))))
      (set `self.ControllerRef` _asbp_player_controller)
      (`PlayerController.SetViewTargetWithBlend` (`self.ControllerRef`) self 0.02 "VTBlend_Linear" 0.0 false)
      (`self.ShowActorWithAttachmentsLocal` (`self.CharacterRef`))
      (`/Game/InteractiveInventory/Blueprints/GameModes-Inventory/BP_PlayerController.EnableUI_Input` (`self.ControllerRef`) true))
    (:`then_1`
      (`KismetSystemLibrary.Delay` 1.3)
      (bind _asbp_hud (cast `/Game/InteractiveInventory/Blueprints/GameModes-Inventory/BP_HUD` (`PlayerController.GetHUD` (`self.ControllerRef`))))
      (bind _output_get (set `self.HUD_Ref` _asbp_hud))
      (`/Game/InteractiveInventory/Blueprints/GameModes-Inventory/BP_HUD.CreateStorageBox` _output_get)
      (if (`KismetSystemLibrary.IsStandalone`)
        (`GameplayStatics.SetGamePaused` true)))))

(event `StorageEnd`
  ;[0.2225 0.1422 1] when you want close storage
  (if (`KismetSystemLibrary.IsStandalone`)
    (`GameplayStatics.SetGamePaused` false))
  (`self.Server_StorageEnd`)
  (`KismetSystemLibrary.Delay` 1.0)
  (`/Game/InteractiveInventory/Blueprints/GameModes-Inventory/BP_PlayerController.EnableUI_Input` (`self.ControllerRef`) false)
  (`PlayerController.SetViewTargetWithBlend` (`self.ControllerRef`) (`self.CharacterRef`) 0.02 "VTBlend_Linear" 0.0 false)
  (`self.ShowActorWithAttachmentsLocal` (`self.CharacterRef`) true)
  (set `self.ControllerRef` null)
  (set `self.HUD_Ref` null))

(event `Server_StorageEnd`
  ;[0.25 0.758 1] Storage end called
  (`/Game/InteractiveInventory/Blueprints/Inventory/Storage/BP_StorageManagerActor.SetActiveStorageRef` (`/Game/InteractiveInventory/Blueprints/Inventory/InventoryManagerLibrary.GetStorageManagerActorRef`) null)
  (`self.SetOwner` null)
  (`self.Mulitcast_OpenCrateDoor` false)
  (`self.EnableInteraction` true))

(event `Mulitcast_OpenCrateDoor`
  (params (Open :type Boolean))
  ;[0.25 0.758 1] cratedoor anim
  (if Open
    (`SkeletalMeshComponent.PlayAnimation` (`self.SKM_MilitaryCrate`) "/Game/InteractiveInventory/Animations/MilitaryCrate/AS_MilitaryCrate_Open.AS_MilitaryCrate_Open" false)
    (else
      (`SkeletalMeshComponent.PlayAnimation` (`self.SKM_MilitaryCrate`) "/Game/InteractiveInventory/Animations/MilitaryCrate/AS_MilitaryCrate_Close.AS_MilitaryCrate_Close" false))))

(fn `StorageBegin`
  (params (CharacterRef :type "Character Object Reference"))
  ;[1 1 1] on interact with storage begins in server
  (`/Game/InteractiveInventory/Blueprints/Inventory/Storage/BP_StorageManagerActor.SetActiveStorageRef` (`/Game/InteractiveInventory/Blueprints/Inventory/InventoryManagerLibrary.GetStorageManagerActorRef`) self)
  (`self.SetOwner` (`local.CharacterRef`))
  (`self.Mulitcast_OpenCrateDoor` true)
  (`self.EnableInteraction` false)
  (`self.Client_StorageBegin` (`local.CharacterRef`)))

(fn `UserConstructionScript`)