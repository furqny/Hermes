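; InventoryManagerLibrary is a function library that gives world-context access to the inventory system's storage, shop and typewriter managers.
; The manager getters cast the game state to BP_GameState and return the manager references stored on it.
; The storage and shop inventory getters build on those, returning each manager's inventory only when the manager is valid.
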(fn `GetShopInventoryRef`
  (returns (Storage :type "/Game/InteractiveInventory/Blueprints/Inventory/BPC_Inventory Object Reference"))
  (locals (ShopRef :type "/Game/InteractiveInventory/Blueprints/Inventory/Shop/BP_ShopManagerActor Object Reference"))
  (bind _output_get (set `local.ShopRef` (`self.GetShopManagerActorRef` (`local.__WorldContext`))))
  (`/Engine/EditorBlueprintResources/StandardMacros.IsValid` _output_get
    (:`Is Valid`
      (return (`/Game/InteractiveInventory/Blueprints/Inventory/Shop/BP_ShopManagerActor.ShopInventory` _output_get)))
    (:`Is Not Valid`
      (return null))))

(fn `GetShopManagerActorRef`
  (returns (ReturnValue :type "/Game/InteractiveInventory/Blueprints/Inventory/Shop/BP_ShopManagerActor Object Reference"))
  (bind _asbp_game_state (cast `/Game/InteractiveInventory/Blueprints/GameModes-Inventory/BP_GameState` (`GameplayStatics.GetGameState` (`local.__WorldContext`))))
  (return (`/Game/InteractiveInventory/Blueprints/GameModes-Inventory/BP_GameState.ShopManagerRef` _asbp_game_state)))

(fn `GetStorageInventoryRef`
  (returns (Storage :type "/Game/InteractiveInventory/Blueprints/Inventory/BPC_Inventory Object Reference"))
  (locals (StorageRef :type "/Game/InteractiveInventory/Blueprints/Inventory/Storage/BP_StorageManagerActor Object Reference"))
  (bind _output_get (set `local.StorageRef` (`self.GetStorageManagerActorRef` (`local.__WorldContext`))))
  (`/Engine/EditorBlueprintResources/StandardMacros.IsValid` _output_get
    (:`Is Valid`
      (return (`/Game/InteractiveInventory/Blueprints/Inventory/Storage/BP_StorageManagerActor.Storage` _output_get)))
    (:`Is Not Valid`
      (return null))))

(fn `GetStorageManagerActorRef`
  (returns (ReturnValue :type "/Game/InteractiveInventory/Blueprints/Inventory/Storage/BP_StorageManagerActor Object Reference"))
  (bind _asbp_game_state (cast `/Game/InteractiveInventory/Blueprints/GameModes-Inventory/BP_GameState` (`GameplayStatics.GetGameState` (`local.__WorldContext`))))
  (return (`/Game/InteractiveInventory/Blueprints/GameModes-Inventory/BP_GameState.StorageManagerRef` _asbp_game_state)))

(fn `GetTypewriterManagerActorRef`
  (returns (TypewriterManagerRef :type "/Game/InteractiveInventory/Blueprints/Saves/BP_TypewriterManagerActor Object Reference"))
  (bind _asbp_game_state (cast `/Game/InteractiveInventory/Blueprints/GameModes-Inventory/BP_GameState` (`GameplayStatics.GetGameState` (`local.__WorldContext`))))
  (return (`/Game/InteractiveInventory/Blueprints/GameModes-Inventory/BP_GameState.TypewriterManagerRef` _asbp_game_state)))