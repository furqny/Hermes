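; Basic inventory item actor that can be picked up through interaction and saved or loaded.
; On interaction, an unowned item passes itself to the interactor's BPC_Inventory; a successful pickup disables further interaction and makes the interactor its owner.
; SaveItem adds the item's class, location and amount to the supplied save reference, and LoadItem restores location and amount from that data.
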(event `self.ReceiveBeginPlay`
  (`parent.ReceiveBeginPlay`))

(event `self.InteractReceived`
  (params (NewOwner :type "Actor Object Reference"))
  (if (not (`KismetSystemLibrary.IsValid` (`self.GetOwner`)))
    (`self.Pickup` NewOwner)))

(fn `LoadItem`
  (params (ItemData :type "/Game/InteractiveInventory/Structure/F_ItemSaveData Structure"))
  (bind ((`Location_2_2D5ED5A34436430AB8DC35AA7204D2AD` _location) (`Amount_5_247968884B7A5BDB034C30BD7DF60C7C` _amount)) (break `/Game/InteractiveInventory/Structure/F_ItemSaveData` ItemData))
  (`self.K2_SetActorLocation` _location)
  (set `self.Amount` _amount))

(fn `Pickup`
  (params (NewOwner :type "Actor Object Reference"))
  (bind _output_get (set `self.InventoryRef_0` (`self.GetComponentByClass` NewOwner "/Game/InteractiveInventory/Blueprints/Inventory/BPC_Inventory.BPC_Inventory_C")))
  (bind _success (`/Game/InteractiveInventory/Blueprints/Inventory/BPC_Inventory.PickupObjectActor` _output_get self))
  (if _success
    (`self.EnableInteraction` false)
    (`self.SetOwner` (`local.NewOwner`))))

(fn `SaveItem`
  (params (ItemSaveRef :type "/Game/InteractiveInventory/Blueprints/Saves/BP_SaveItem Object Reference"))
  (locals (LocalSaveRef :type "/Game/InteractiveInventory/Blueprints/Saves/BP_SaveWeapon Object Reference"))
  (`/Game/InteractiveInventory/Blueprints/Saves/BP_SaveItem.AddItem` ItemSaveRef (make `/Game/InteractiveInventory/Structure/F_ItemSaveData` (`GameplayStatics.GetObjectClass` self) (`self.K2_GetActorLocation`) (`self.Amount`))))

(fn `UserConstructionScript`)