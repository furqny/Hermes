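; Base actor for advanced inventory items such as weapons, with networked pickup, equip, drop, upgrade and save support.
; Interacting with an unowned item goes through BPC_Inventory, then pickup attaches it hidden to a character socket.
; Server and client events split visibility, input and HUD changes.
; Upgrades apply UpgradeList levels and spend gold on the server, while child classes override placeholder attribute, item HUD and save/load functions.
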(event `self.InteractReceived`
  (params (NewOwner :type "Actor Object Reference"))
  ;[0.247 1 0.1257] Interact
  (`/Engine/EditorBlueprintResources/StandardMacros.IsValid` (`self.GetOwner`)
    (:`Is Not Valid`
      (bind _success (`/Game/InteractiveInventory/Blueprints/Inventory/BPC_Inventory.PickupObjectActor` (`self.GetComponentByClass` NewOwner "/Game/InteractiveInventory/Blueprints/Inventory/BPC_Inventory.BPC_Inventory_C") self))
      (if _success
        (`self.SetOwner` NewOwner)
        (`self.EnableInteraction` false)))))

(event `self.ReceiveBeginPlay`
  (`parent.ReceiveBeginPlay`)
  (bind _returnvalue (`|CreateWidget` "/Game/InteractiveInventory/Blueprints/UI/HUD/WBP_E_Widget.WBP_E_Widget_C"))
  (set `self.Widget_Ref` _returnvalue))

(event `Clinet_OnControllerChanged`
  (params (NewControllerPawn :type "Pawn Object Reference"))
  ;[0.25 0.758 1] On pick up completed, handle some setting in client
  (bind _asplayer_controller (cast `PlayerController` (`Pawn.GetController` NewControllerPawn)))
  (bind _output_get (set `self.PlayerControllerRef` _asplayer_controller))
  (bind _asbp_hud (cast `/Game/InteractiveInventory/Blueprints/GameModes-Inventory/BP_HUD` (`PlayerController.GetHUD` _output_get)))
  (set `self.HUD_Ref` _asbp_hud))

(event `Client_UnequipItem`
  ;[0.25 0.758 1] Hide the actor on server when unequip
  (if (`self.IsEquipped`)
    (set `self.IsEquipped` false)
    (`self.HideItemHUD_Widget`)
    (`/Game/InteractiveInventory/Blueprints/GameModes-Inventory/BP_HUD.HideCrosshair` (`self.HUD_Ref`))
    (`self.DisableInput` (`self.PlayerControllerRef`))
    (`self.SetActorTickEnabled` false)))

(event `Server_EquipCompleted`
  ;[1 1 1] Server
  (`self.SetActorHiddenInGame` false))

(event `Client_DropItem`
  ;[0.25 0.758 1] On item Dropped in client
  (`self.SetActorTickEnabled` false)
  (`self.HideItemHUD_Widget`)
  (`/Game/InteractiveInventory/Blueprints/GameModes-Inventory/BP_HUD.HideCrosshair` (`self.HUD_Ref`))
  (`self.DisableInput` (`self.PlayerControllerRef`))
  (set `self.PlayerControllerRef` null)
  (set `self.HUD_Ref` null))

(event `Server_UnequipCompleted`
  ;[1 1 1] Server
  (`self.SetActorHiddenInGame` true))

(event `Client_UpgradeCompleted`
  ;[0.25 0.758 1] on upgrade completed, changes visual and audial for client
  (`self.UpgradeCompletedWidget`)
  (`/Game/InteractiveInventory/Blueprints/GameModes-Inventory/BP_HUD.UpdateShop` (`self.HUD_Ref`)))

(event `self.ReceiveDestroyed`
  ;[0.724 0.09049 0.09049] On Destroyed
  (`self.HideItemHUD_Widget`)
  (`parent.ReceiveDestroyed`))

(event `Server_UpgradeItem`
  (params (UpgradeIndex :type Integer))
  ;[0.25 0.758 1] Handle Upgrade On Server
  (`self.HandleUpgrade` UpgradeIndex))

(fn `ChangeOwner`
  (params (NewOwner :type "Actor Object Reference"))
  (`self.SetOwner` NewOwner))

(fn `DropItem`
  (bind _returnvalue_location (`KismetMathLibrary.BreakTransform` (`self.GetTransform` (`self.CharacterRef`))))
  ;[1 1 1] Handle settings for droping item on server
  (`self.SetActorHiddenInGame` false)
  (`self.K2_SetActorLocation` (+ _returnvalue_location (* (`self.GetActorForwardVector` (`self.CharacterRef`)) 150.0)) false true)
  (`PrimitiveComponent.SetCollisionEnabled` (`self.InteractBox`) "QueryOnly")
  (`self.K2_DetachFromActor` "KeepWorld" "KeepWorld" "KeepWorld")
  (`PrimitiveComponent.SetSimulatePhysics` (`self.ItemSkeletalMesh`) true)
  (set `self.CharacterRef` null)
  (`self.Client_DropItem`)
  (`self.EnableInteraction` true)
  (`self.SetOwner` null))

(fn `EquipCompleted`
  (if (not (`self.IsEquipped`))
    (set `self.IsEquipped` true)
    (`self.Server_EquipCompleted`)
    (`self.SetActorTickEnabled` true)
    (`self.EnableInput` (`self.PlayerControllerRef`))
    (`self.ShowItemHUD`)
    (`self.SetActorHiddenInGame` false)))

(fn `GetCurrentAttribute`
  (params (UpgradeMode :type "/Game/InteractiveInventory/Enum/E_UpgradeType Enum" :default "NewEnumerator0"))
  (returns (ReturnValue :type "Float (double-precision)"))
  ;[1 0.8124 0] Please Override this function
  ; add your own variable in there
  (`KismetSystemLibrary.LogString` "Please Override this function \nadd your own variable in there")
  (return 0.0))

(fn `HandleUpgrade`
  (params (UpgradeIndex :type Integer))
  (locals (SelectedUpgrade :type "/Game/InteractiveInventory/Structure/F_UpgradeList Structure"))
  (bind (_output_upgradetype _output_upgrades _output_currentlevel) (break `/Game/InteractiveInventory/Structure/F_UpgradeList` (`|GetArrayItem` (`self.UpgradeList`) UpgradeIndex)))
  (bind (_output_level _output_newamount _output_price) (break `/Game/InteractiveInventory/Structure/F_UpgradeDetails` (`|GetArrayItem` _output_upgrades _output_currentlevel)))
  ;[1 1 1] Upgrade item (Like Weapon) to the new level
  (`self.SetAttribute` _output_upgradetype _output_newamount)
  (`/Game/InteractiveInventory/Blueprints/Inventory/BPC_Inventory.UseGold` (`self.InventoryRef_0`) _output_price)
  (`KismetArrayLibrary.Array_Set` (`self.UpgradeList`) (`local.UpgradeIndex`) (make `/Game/InteractiveInventory/Structure/F_UpgradeList` _output_upgradetype _output_upgrades (+ _output_currentlevel 1)))
  (`self.Client_UpgradeCompleted`))

(fn `HideItemHUD_Widget`
  ;[1 0.7657 0] Please Override this function
  ; add your own variable in there
  (`KismetSystemLibrary.LogString` "Please Override this function \nadd your own variable in there"))

(fn `LoadActorData`
  (params (Data :type "/Game/InteractiveInventory/Structure/F_AdvanceItemsDetails Structure"))
  ;[1 0.8124 0] Please Override this function
  ; add your own variable in there
  (`KismetSystemLibrary.LogString` "Please Override this function \nadd your own variable in there"))

(fn `OnPickupCompleted`
  (params (InNewOwner :type "Actor Object Reference"))
  ;[1 1 1] When pickup Completed, this item will be added to inventory
  (`self.SetOwner` (`local.InNewOwner`))
  (`PrimitiveComponent.SetSimulatePhysics` (`self.ItemSkeletalMesh`) false)
  (`PrimitiveComponent.SetSimulatePhysics` (`self.ItemStaticMesh`) false)
  (`PrimitiveComponent.SetCollisionEnabled` (`self.InteractBox`) "NoCollision")
  (`self.SetActorHiddenInGame` true)
  (bind _ascharacter (cast `Character` (`local.InNewOwner`)))
  (bind _output_get (set `self.CharacterRef` _ascharacter))
  (`self.K2_AttachToComponent` (`Character.Mesh` _output_get) (`self.AttachSocketName`) "SnapToTarget" "SnapToTarget" "KeepWorld")
  (set `self.InventoryRef_0` (`self.GetComponentByClass` (`self.CharacterRef`) "/Game/InteractiveInventory/Blueprints/Inventory/BPC_Inventory.BPC_Inventory_C"))
  (`self.Clinet_OnControllerChanged` (`self.CharacterRef`))
  (`self.EnableInteraction` false))

(fn `SaveActorData`
  (params (SaveGameRef :type "SaveGame Object Reference") (IndexInInventory :type Integer))
  (bind _asbp_save_weapon (cast `/Game/InteractiveInventory/Blueprints/Saves/BP_SaveWeapon` SaveGameRef))
  (`/Game/InteractiveInventory/Blueprints/Saves/BP_SaveWeapon.AddWeapon` _asbp_save_weapon (make `/Game/InteractiveInventory/Structure/F_AdvanceSave` (`GameplayStatics.GetObjectClass` self) (`self.K2_GetActorLocation`) IndexInInventory (make `/Game/InteractiveInventory/Structure/F_AdvanceItemsDetails` 0.0)))
  (`KismetSystemLibrary.PrintString` "Override \"saveActorData\"and write save code"))

(fn `SetAttribute`
  (params (UpgradeType :type "/Game/InteractiveInventory/Enum/E_UpgradeType Enum" :default "NewEnumerator0") (NewAttribute :type "Float (double-precision)"))
  ;[1 0.8124 0] Please Override this function
  ; add your own variable in there
  (`KismetSystemLibrary.LogString` "Please Override this function \nadd your own variable in there"))

(fn `ShowItemHUD`
  ;[1 0.8124 0] Please Override this function
  ; add your own variable in there
  (`KismetSystemLibrary.LogString` "Please Override this function \nadd your own variable in there"))

(fn `UnequipCompleted`
  ;[1 1 1] on item unequipped
  (if (`self.IsEquipped`)
    (set `self.IsEquipped` false)
    (`self.Server_UnequipCompleted`)
    (`self.SetActorHiddenInGame` true)
    (`self.HideItemHUD_Widget`)
    (`/Game/InteractiveInventory/Blueprints/GameModes-Inventory/BP_HUD.HideCrosshair` (`self.HUD_Ref`))
    (`self.DisableInput` (`self.PlayerControllerRef`))
    (`self.SetActorTickEnabled` false)))

(fn `UpdateObjectWidget`
  (bind _hud_ref (`self.HUD_Ref`))
  (`/Game/InteractiveInventory/Blueprints/GameModes-Inventory/BP_HUD.UpdateAmmo` _hud_ref)
  (`/Game/InteractiveInventory/Blueprints/GameModes-Inventory/BP_HUD.UpdateInventoryMenu` _hud_ref))

(fn `UpgradeCompletedWidget`
  (bind ((`ItemName_8_08C08377453A03C483C2CDA91290553A` _itemname) (`Image_18_D704C90842707B714A2C6CB0C5AE694A` _image)) (break `/Game/InteractiveInventory/Structure/F_ItemDetails` (`/Game/InteractiveInventory/Blueprints/Inventory/BPC_Inventory.GetObjectDetails` (`self.InventoryRef_0`) (`GameplayStatics.GetObjectClass` self))))
  ;[1 1 1] On Upgrade Completed, show completed upgrade widget
  (`/Game/InteractiveInventory/Blueprints/GameModes-Inventory/BP_HUD.AddNewInfo` (`self.HUD_Ref`) (`KismetTextLibrary.Conv_StringToText` (`KismetStringLibrary.Concat_StrStr` (`KismetTextLibrary.Conv_TextToString` _itemname) " Upgrade Completed")) _image (struct :`R` 0.8 :`G` 0.8 :`B` 1.0 :`A` 1.0)))

(fn `UpgradeItem`
  (params (UpgradeIndex :type Integer) (UpgradeWidgetRef :type "UserWidget Object Reference"))
  ;[1 1 1] Upgrade
  (`self.Server_UpgradeItem` UpgradeIndex)
  (if (not (`KismetSystemLibrary.IsStandalone`))
    (`/Engine/EditorBlueprintResources/ActorMacros.Switch Has Authority`
      (:`Remote`
        (`/Game/InteractiveInventory/Blueprints/GameModes-Inventory/BP_HUD.ShowServerResponse` (`self.HUD_Ref`) (`local.UpgradeWidgetRef`))))))

(fn `UserConstructionScript`)