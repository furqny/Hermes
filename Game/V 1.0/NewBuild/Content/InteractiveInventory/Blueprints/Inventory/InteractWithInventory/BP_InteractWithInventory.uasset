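; Interactable lock actor that lets one character at a time interact with it through their inventory, with server and client handling.
; On interact, it takes the character as owner, disables further interaction, and has the client switch view to it, hide the character and open an interact widget after a delay.
; Ending interaction restores the view, input and availability, and clears ownership.
; CheckKey is an empty stub.
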(event `self.InteractReceived`
  (params (NewOwner :type "Actor Object Reference"))
  ;[0.945 1 0.5841] Start Interact with Lock
  (`/Engine/EditorBlueprintResources/StandardMacros.IsValid` (`self.GetOwner`)
    (:`Is Not Valid`
      (`self.StartInteraction` NewOwner))))

(event `Client_StartInteract`
  (params (CharacterRef :type "Character Object Reference"))
  ;[1 1 1] Start interaction on client
  (set `self.CharacterRef` CharacterRef)
  (`|ExecutionSequence`
    (:`then_0`
      (set `self.InventoryRef_0` (`self.GetComponentByClass` (`self.CharacterRef`) "/Game/InteractiveInventory/Blueprints/Inventory/BPC_Inventory.BPC_Inventory_C"))
      (set `/Game/InteractiveInventory/Blueprints/Inventory/BPC_Inventory.ActiveLockRef` self (`self.InventoryRef_0`)))
    (:`then_1`
      (bind _asbp_player_controller (cast `/Game/InteractiveInventory/Blueprints/GameModes-Inventory/BP_PlayerController` (`Pawn.GetController` (`self.CharacterRef`))))
      (set `self.ControllerRef` _asbp_player_controller)
      (`PlayerController.SetViewTargetWithBlend` (`self.ControllerRef`) self 0.02 "VTBlend_Linear" 0.0 false)
      (`self.ShowActorWithAttachmentsLocal` (`self.CharacterRef`))
      (`/Game/InteractiveInventory/Blueprints/GameModes-Inventory/BP_PlayerController.EnableUI_Input` (`self.ControllerRef`) true))
    (:`then_2`
      (`KismetSystemLibrary.Delay` 0.4)
      (bind _asbp_hud (cast `/Game/InteractiveInventory/Blueprints/GameModes-Inventory/BP_HUD` (`PlayerController.GetHUD` (`self.ControllerRef`))))
      (bind _output_get (set `self.HUD_Ref` _asbp_hud))
      (`/Game/InteractiveInventory/Blueprints/GameModes-Inventory/BP_HUD.CreateInteractwidget` _output_get self))))

(event `Client_InteractionEnd`
  ;[1 1 1] Interaction end on Client
  (`/Game/InteractiveInventory/Blueprints/GameModes-Inventory/BP_HUD.HideInteractWidget` (`self.HUD_Ref`))
  (`/Game/InteractiveInventory/Blueprints/GameModes-Inventory/BP_PlayerController.EnableUI_Input` (`self.ControllerRef`) false)
  (`PlayerController.SetViewTargetWithBlend` (`self.ControllerRef`) (`self.CharacterRef`) 0.02 "VTBlend_Linear" 0.0 false)
  (`self.ShowActorWithAttachmentsLocal` (`self.CharacterRef`) true))

(event `Server_InteractionEnd`
  ;[0.25 0.758 1] Interaction end on server
  (`self.EnableInteraction` true)
  (`self.Client_InteractionEnd`)
  (`self.SetOwner` null)
  (set `/Game/InteractiveInventory/Blueprints/Inventory/BPC_Inventory.ActiveLockRef` null (`self.InventoryRef_0`)))

(fn `CheckKey`
  (params (KeyActor :type "Actor Class Reference"))
  (locals (AcceptedActor :type "/Game/InteractiveInventory/Blueprints/Interact/BP_Interactable Object Reference")))

(fn `InteractionEnd`
  (`self.Server_InteractionEnd`))

(fn `StartInteraction`
  (params (NewOwner :type "Actor Object Reference"))
  (bind _ascharacter (cast `Character` NewOwner))
  (bind _output_get (set `self.CharacterRef` _ascharacter))
  (bind _output_get_2 (set `self.InventoryRef_0` (`self.GetComponentByClass` _output_get "/Game/InteractiveInventory/Blueprints/Inventory/BPC_Inventory.BPC_Inventory_C")))
  (`/Engine/EditorBlueprintResources/StandardMacros.IsValid` _output_get_2
    (:`Is Valid`
      (`self.SetOwner` (`self.CharacterRef`))
      (`self.EnableInteraction` false)
      (`self.Client_StartInteract` (`self.CharacterRef`)))
    (:`Is Not Valid`
      (`KismetSystemLibrary.PrintString` "Interaction BPC Missing on the character"))))

(fn `UserConstructionScript`)