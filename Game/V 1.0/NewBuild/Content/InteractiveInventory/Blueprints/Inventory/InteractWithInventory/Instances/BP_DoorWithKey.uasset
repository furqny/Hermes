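; Double door in the interactive inventory system that stays locked until the required key item is used on it.
; While locked, interaction defers to the parent; CheckKey compares item class, and a match triggers a server event that optionally consumes the item, unlocks and opens the door.
; Once unlocked, interaction sets the owner and toggles a multicast timeline that swings both leaves open or closed.
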(event `self.InteractReceived`
  (params (NewOwner :type "Actor Object Reference"))
  (if (`self.bIsUnlocked`)
    (`self.SetOwner` NewOwner)
    (`self.Multicast_OpenDoor` (not (`self.bIsOpening`)))
    (else
      (`parent.InteractReceived` NewOwner))))

(event `Server_KeyAccepted`
  ;[1 1 1] Comment
  (`self.KeyAccepted`))

(event `Multicast_OpenDoor`
  (params (OpenDoor :type Boolean))
  ;[1 1 1] OpenDoorAnim
  (if OpenDoor
    (set `self.bIsOpening` true)
    (bind (_direction _door) (`Timeline|Timeline` :!label _label)
      (:`Update`
        (`SceneComponent.K2_SetRelativeRotation` (`self.Door1`) (`KismetMathLibrary.MakeRotator` 0.0 0.0 (`KismetMathLibrary.Lerp` 180.0 90.0 _door)) false true)
        (`SceneComponent.K2_SetRelativeRotation` (`self.Door2`) (`KismetMathLibrary.MakeRotator` 0.0 0.0 (`KismetMathLibrary.Lerp` 0.0 90.0 _door)) false true))
      (:`Finished`
        (`/Engine/EditorBlueprintResources/ActorMacros.Switch Has Authority`
          (:`Authority`
            (`self.SetOwner` null)))))
    (else
      (set `self.bIsOpening` false)
      (goto _label :!via `Reverse`))))

(fn `CheckKey`
  (params (KeyActor :type "Actor Class Reference"))
  (if (`KismetMathLibrary.ClassIsChildOf` (`self.RequiredItem`) KeyActor)
    (`self.Server_KeyAccepted`)
    (else
      (`KismetSystemLibrary.PrintString` "cant use this"))))

(fn `KeyAccepted`
  (`|ExecutionSequence`
    (:`then_0`
      (switch `/Game/InteractiveInventory/Enum/E_InventoryInteractionMode` (`self.InventoryInteractionMode`)
        (:`NewEnumerator0`
          (`/Game/InteractiveInventory/Blueprints/Inventory/BPC_Inventory.ReduceItem` (`self.InventoryRef_0`) (`self.RequiredItem`) 1))))
    (:`then_1`
      (set `self.bIsUnlocked` true)
      (`self.Multicast_OpenDoor` true))
    (:`then_2`
      (`self.Server_InteractionEnd`))))

(fn `UserConstructionScript`
  (`parent.UserConstructionScript`))