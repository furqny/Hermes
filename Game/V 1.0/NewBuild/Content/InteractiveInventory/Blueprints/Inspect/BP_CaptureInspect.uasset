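; Scene-capture actor for the inventory's item inspect view, rendering only the inspected mesh while the HUD creates the inspect widget.
; SetItemToInspect swaps the mesh, activates the capture and plays a timeline blending it to the target scale and rotation.
; Tick eases rotation toward a clamped angle derived from mouse offset from viewport center.
; Flip turns the item around, the wheel zooms via capture FOV, and QuitInspect disables capture, tick and input.
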(event `self.ReceiveBeginPlay`
  ;[0.945 1 0.5841] At Start, set the target static mesh
  (`SceneCaptureComponent.ShowOnlyComponent` (`self.SceneCaptureComponent2D`) (`self.ItemStaticMesh`)))

(event `self.ReceiveTick`
  (params (DeltaSeconds :type "Float (single-precision)"))
  ;[0.945 1 0.5841] Tick Update every frame
  (`self.CalculateItemInWidgetRotation`)
  (`SceneComponent.K2_SetRelativeRotation` (`self.ItemStaticMesh`) (`KismetMathLibrary.RInterpTo` (`SceneComponent.RelativeRotation` (`self.ItemStaticMesh`)) (`self.ItemTargetRotation`) DeltaSeconds 14.0) false true))

(event `Flip`
  ;[1 0.4875 0.9353] Flip the inspected Item
  (`/Engine/EditorBlueprintResources/StandardMacros.FlipFlop`
    (:`A`
      (set `self.FlipItem` true))
    (:`B`
      (set `self.FlipItem` false))))

(event `QuitInspect`
  ;[1 0.4875 0.9353] QuitInspect
  (`ActorComponent.Deactivate` (`self.SceneCaptureComponent2D`))
  (`self.SetActorTickEnabled` false)
  (`self.DisableInput` (`self.PlayerControllerRef`)))

(event `CreateInspectWidget`
  (params (InspectText :type Text))
  ;[1 0.4875 0.9353] Create The inspect Widget
  (bind _asbp_hud (cast `/Game/InteractiveInventory/Blueprints/GameModes-Inventory/BP_HUD` (`PlayerController.GetHUD` (`self.PlayerControllerRef`))))
  (`/Game/InteractiveInventory/Blueprints/GameModes-Inventory/BP_HUD.CreateInspectWidget` _asbp_hud InspectText))

(event `SetItemToInspect`
  (params (ItemMesh :type "StaticMesh Object Reference") (Pawn :type "Pawn Object Reference") (InspectText :type Text) (TargetScale :type "Vector Structure"))
  ;[1 1 1] Item Comes to Player inspcet
  (bind _asplayer_controller (cast `PlayerController` (`Pawn.GetController` Pawn))
    (:`then`
      (set `self.Var_InspectScale` TargetScale)
      (set `self.PlayerControllerRef` _asplayer_controller))
    (:`CastFailed`
      _))
  (set `self.FlipItem` false)
  (`StaticMeshComponent.SetStaticMesh` (`self.ItemStaticMesh`) ItemMesh)
  (`self.CreateInspectWidget` InspectText)
  (`self.SetActorTickEnabled` true)
  (`ActorComponent.Activate` (`self.SceneCaptureComponent2D`) false)
  (`|ExecutionSequence`
    (:`then_0`
      (bind (_direction _alphaa) (`Timeline|Timeline` :!via `SetNewTime` :!label _label)
        (:`Update`
          (`self.CalculateItemInWidgetRotation`)
          (`SceneComponent.K2_SetRelativeTransform` (`self.ItemStaticMesh`) (`KismetMathLibrary.TLerp` (`self.InspectItemTransform`) (`KismetMathLibrary.MakeTransform` (0.0 0.0 0.0) (`self.ItemTargetRotation`) (`self.Var_InspectScale`)) _alphaa "EulerInterp") false false))
        (:`Finished`
          (`self.SetActorTickEnabled` true)
          (`self.EnableInput` (`self.PlayerControllerRef`)))))
    (:`then_1`
      (goto _label))))

(event `SetItemPositionToDefault`
  ;[1 1 1] Item Comes to Player inspcet
  (goto _label :!via `Stop`))

(event `WheelAxis`
  (params (AxisValue :type "Float (double-precision)"))
  ;[1 1 1] Zoom
  (set `SceneCaptureComponent2D.FOVAngle` (`KismetMathLibrary.FClamp` (+ (`SceneCaptureComponent2D.FOVAngle` (`self.SceneCaptureComponent2D`)) (* AxisValue 1.0)) 30.0 110.0) (`self.SceneCaptureComponent2D`)))

(fn `ApplyLimit`
  (params (Offset :type "Float (double-precision)") (Value :type "Float (double-precision)"))
  (returns (ReturnValue :type "Float (double-precision)"))
  (bind _itemrotationlimit (`self.ItemRotationLimit`))
  (bind _returnvalue (* (`KismetMathLibrary.FClamp` (/ Value 10.0) (* _itemrotationlimit -1.0) _itemrotationlimit) -1.0))
  ;[1 1 1] Apply limit to the rotation of the object
  (return (`KismetMathLibrary.SelectFloat` (+ Offset _returnvalue) _returnvalue (`self.FlipItem`))))

(fn `CalculateItemInWidgetRotation`
  (bind (_returnvalue_x _returnvalue_y) (`KismetMathLibrary.BreakVector2D` (`WidgetLayoutLibrary.GetViewportSize`)))
  (bind (_returnvalue_x_2 _returnvalue_y_2) (`KismetMathLibrary.BreakVector2D` (`WidgetLayoutLibrary.GetViewportSize`)))
  (bind (_x _y) (`KismetMathLibrary.BreakVector2D` (`self.LastMousePosition`)))
  (bind (_x_2 _y_2) (`KismetMathLibrary.BreakVector2D` (- (`self.NewMousePosition`) (`KismetMathLibrary.MakeVector2D` (/ _returnvalue_x 2.0) (/ _returnvalue_y 2.0)))))
  (bind _returnvalue (`self.ApplyLimit` 0.0 _y_2))
  ;[1 1 1] Depends on the mouse position of the mouse, set the new rotation of the object
  (bind _returnvalue_2 (`WidgetLayoutLibrary.GetMousePositionOnViewport`))
  (bind (_x_3 _y_3) (`KismetMathLibrary.BreakVector2D` _returnvalue_2))
  (set `self.NewMousePosition` (`KismetMathLibrary.MakeVector2D` (`self.CalculateMousePositionX/Y` _returnvalue_x_2 _x_3 _x) (`self.CalculateMousePositionX/Y` _returnvalue_y_2 _y_3 _y)))
  (set `self.ItemTargetRotation` (`KismetMathLibrary.MakeRotator` (`KismetMathLibrary.SelectFloat` _returnvalue (* _returnvalue -1.0) (`self.FlipItem`)) 0.0 (`self.ApplyLimit` 179.0 _x_2))))

(fn `CalculateMousePositionX/Y`
  (params (`ViewportSizeX/Y` :type "Float (double-precision)") (`CurrentMouseLocationX/Y` :type "Float (double-precision)") (`LastMouseLocationX/Y` :type "Float (double-precision)"))
  (returns (Output :type "Float (double-precision)"))
  (bind _returnvalue (`KismetMathLibrary.SelectFloat` (`local.ViewportSizeX/Y`) (`local.CurrentMouseLocationX/Y`) (>= (`local.CurrentMouseLocationX/Y`) (`local.ViewportSizeX/Y`))))
  ;[1 1 1] calculate the rotation for one direction of mouse
  (return (`KismetMathLibrary.Conv_IntToDouble` (`KismetMathLibrary.Round` (`KismetMathLibrary.SelectFloat` (`local.LastMouseLocationX/Y`) _returnvalue (`KismetMathLibrary.NearlyEqual_FloatFloat` _returnvalue (`local.LastMouseLocationX/Y`) 4.0))))))

(fn `UserConstructionScript`)