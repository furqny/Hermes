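; Interactable save typewriter actor that opens the save list UI for the character using it, optionally restricted to the host.
; SaveBegin registers it with the typewriter manager as a single-user lock, disables interaction and sets ownership for the client call.
; The client switches view target to the typewriter, hides the character locally, shows the HUD widget and pauses in standalone.
; SaveEnd reverses this and releases the lock through a server event.
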(event `self.ReceiveBeginPlay`
  (`parent.ReceiveBeginPlay`))

(event `self.ReceiveTick`
  (params (DeltaSeconds :type "Float (single-precision)")))

(event `self.InteractReceived`
  (params (NewOwner :type "Actor Object Reference"))
  (bind _ascharacter (cast `Character` NewOwner :!pure true))
  (if (`self.bOnlyHostCanSave`)
    (if (`self.HasAuthority` _ascharacter)
      (`self.SaveBegin` _ascharacter :!label _label)
      (else
        (`KismetSystemLibrary.PrintString` "Only Server Can Save the game")))
    (else
      (goto _label))))

(event `Client_InteractTypewriter`
  (params (CharacterRef :type "Character Object Reference"))
  ;[0.25 0.758 1] get required references and then create widget in HUD
  (set `self.CharacterRef` CharacterRef)
  (`|ExecutionSequence`
    (:`then_0`
      (bind _asbp_player_controller (cast `/Game/InteractiveInventory/Blueprints/GameModes-Inventory/BP_PlayerController` (`Pawn.GetController` (`self.CharacterRef`))))
      (bind _output_get (set `self.PlayerControllerRef` _asbp_player_controller))
      (`/Game/InteractiveInventory/Blueprints/GameModes-Inventory/BP_PlayerController.EnableUI_Input` _output_get true)
      (`PlayerController.SetViewTargetWithBlend` (`self.PlayerControllerRef`) self 0.01 "VTBlend_Linear" 0.0 false)
      (`self.ShowActorWithAttachmentsLocal` (`self.CharacterRef`)))
    (:`then_1`
      (bind _asbp_hud (cast `/Game/InteractiveInventory/Blueprints/GameModes-Inventory/BP_HUD` (`PlayerController.GetHUD` (`self.PlayerControllerRef`))))
      (set `self.HudRef` _asbp_hud)
      (`/Game/InteractiveInventory/Blueprints/GameModes-Inventory/BP_HUD.ShowSaveListWidget` (`self.HudRef`) "NewEnumerator0")
      (`KismetSystemLibrary.Delay` 0.02)
      (if (`KismetSystemLibrary.IsStandalone`)
        (`GameplayStatics.SetGamePaused` true)))))

(event `SaveEnd`
  ;[0.2225 0.1422 1] when you want close storage
  (if (`KismetSystemLibrary.IsStandalone`)
    (`GameplayStatics.SetGamePaused` false))
  (`self.Server_SaveEnd`)
  (`/Game/InteractiveInventory/Blueprints/GameModes-Inventory/BP_PlayerController.EnableUI_Input` (`self.PlayerControllerRef`) false)
  (`KismetSystemLibrary.PrintString` "ddddddddddddddddddddd")
  (`PlayerController.SetViewTargetWithBlend` (`self.PlayerControllerRef`) (`self.CharacterRef`) 0.0 "VTBlend_Linear" 0.0 false)
  (`self.ShowActorWithAttachmentsLocal` (`self.CharacterRef`) true)
  (set `self.PlayerControllerRef` null)
  (set `self.HudRef` null))

(event `Server_SaveEnd`
  ;[0.25 0.758 1] Storage end called
  (`/Game/InteractiveInventory/Blueprints/Saves/BP_TypewriterManagerActor.SetTyperwriterRef` (`/Game/InteractiveInventory/Blueprints/Inventory/InventoryManagerLibrary.GetTypewriterManagerActorRef`) null)
  (`self.SetOwner` null)
  (`self.EnableInteraction` true))

(fn `SaveBegin`
  (params (Character :type "Character Object Reference"))
  (`/Engine/EditorBlueprintResources/StandardMacros.IsValid` (`/Game/InteractiveInventory/Blueprints/Saves/BP_TypewriterManagerActor.TypewriterRef` (`/Game/InteractiveInventory/Blueprints/Inventory/InventoryManagerLibrary.GetTypewriterManagerActorRef`))
    (:`Is Not Valid`
      (`self.EnableInteraction` false)
      (`self.SetOwner` (`local.Character`))
      (`self.Client_InteractTypewriter` (`local.Character`))
      (`/Game/InteractiveInventory/Blueprints/Saves/BP_TypewriterManagerActor.SetTyperwriterRef` (`/Game/InteractiveInventory/Blueprints/Inventory/InventoryManagerLibrary.GetTypewriterManagerActorRef`) self))))

(fn `UserConstructionScript`)