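; Game instance that acts as a global hub for karma score, puzzle progress and world events.
; Simple events relay to dispatchers for element raises, puzzle gates, barriers and the courage stone, or toggle a bird collision flag.
; When GrandRockRaise equals four, PandoraBarrierGone chains the Wisdom and barrier-opening cinematics through finish callbacks, then broadcasts ShieldGone2.
; Karma updates accumulate into a global score, with debug printing or change broadcasting.
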(event `Update Karma`
  (params (Amount :type Integer))
  (bind _output_get (set `self.GlobalKarmaScore` (+ Amount (`self.GlobalKarmaScore`))))
  (`KismetSystemLibrary.PrintString` (`KismetStringLibrary.Conv_IntToString` _output_get)))

(event `PandoraBarrierGone`
  (if (== (`self.GrandRockRaise`) 4)
    (`KismetSystemLibrary.PrintString` "GELDI")
    (bind (_outactor _returnvalue) (`LevelSequencePlayer.CreateLevelSequencePlayer` "/Game/Wisdom_Cinematic.Wisdom_Cinematic"))
    (`MovieSceneSequencePlayer.Play` _returnvalue)
    (add `MovieSceneSequencePlayer.OnFinished` _returnvalue (delegate `Wisdom`))))

(event `Wisdom`
  (bind (_outactor _returnvalue) (`LevelSequencePlayer.CreateLevelSequencePlayer` "/Game/Barrier_Open_Cinematic.Barrier_Open_Cinematic"))
  (`MovieSceneSequencePlayer.Play` _returnvalue)
  (add `MovieSceneSequencePlayer.OnFinished` _returnvalue (delegate `GoneBarrier`)))

(event `MoonRaise`
  (`self.MoonRaiseDispatcher`))

(event `WindRaise`
  (`self.WindRaiseDispatcher`))

(event `GoneBarrier`
  (`self.ShieldGone2`))

(event `UpdateKarma`
  (params (Amount :type Integer))
  (bind _output_get (set `self.GlobalKarmaScore` (+ Amount (`self.GlobalKarmaScore`))))
  (`self.OnKarmaChanged` _output_get))

(event `FireRaise`
  (`self.FireRaiseDispatcher`))

(event `SunRaise`
  (`self.SunRaiseDispatcher`))

(event `BirdCollisionEnable`
  (set `self.BirdCollisionBool` true))

(event `PlatformBarrierBroke`
  (`self.PlatformBarrierGo`))

(event `BirdCollisionDisable`
  (set `self.BirdCollisionBool` false))

(event `CourageTrigger`
  (`self.CourageStonePosition`))

(event `WallPuzzleGateOpen`
  (`self.WallPuzzleSolved`))

(event `ButtonPuzzleGateOpen`
  (`self.ButtonPuzzleSolved`))