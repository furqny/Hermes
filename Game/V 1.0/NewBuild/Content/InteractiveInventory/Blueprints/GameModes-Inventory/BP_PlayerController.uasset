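; Player controller that lets the third-person character possess bird statues and return to its own body.
; While the game instance's bird flag is set, Tick sphere-traces forward and outlines actors with a Possess component.
; IA_Possess plays a magic-circle effect and montage, swaps the statue's mesh and material, then possesses it.
; IA_Return fades the camera, restores the statue and repossesses the starting pawn; a helper toggles UI-only input.
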(event `self.ReceiveBeginPlay`
  (set `self.StartingControl` (`self.K2_GetPawn`)))

(event `self.ReceiveTick`
  (params (DeltaSeconds :type "Float (single-precision)"))
  (bind _possesableobject (`self.PossesableObject`))
  (bind _returnvalue (`self.GetComponentByClass` (`self.K2_GetPawn`) "/Script/Engine.CapsuleComponent"))
  (bind _returnvalue_2 (`SceneComponent.K2_GetComponentLocation` _returnvalue))
  (if (`self.Isbirdpossesed`)
    (`self.K2_SetActorRotation` (`KismetMathLibrary.MakeRotator` 0.0 0.0 (.yaw (`KismetMathLibrary.FindLookAtRotation` (`self.K2_GetActorLocation` (`GameplayStatics.GetPlayerCharacter` 0)) (`self.K2_GetActorLocation` (`self.PossesableObject`)))))))
  (bind _asbp_main_game_instance (cast `/Game/InteractiveInventory/Blueprints/GameModes-Inventory/BP_MainGameInstance` (`GameplayStatics.GetGameInstance`)))
  (if (`/Game/InteractiveInventory/Blueprints/GameModes-Inventory/BP_MainGameInstance.BirdCollisionBool` _asbp_main_game_instance)
    (bind (_outhit _returnvalue_3) (`KismetSystemLibrary.SphereTraceSingle` :`Start` _returnvalue_2 :`End` (+ _returnvalue_2 (* (`SceneComponent.GetForwardVector` _returnvalue) 2000.0)) :`Radius` 35.0 :`TraceChannel` "TraceTypeQuery1" :`bTraceComplex` true :`DrawDebugType` "ForOneFrame"))
    (if _returnvalue_3
      (bind _asbp_third_person_character (cast `/Game/InteractiveInventory/Blueprints/GameModes-Inventory/BP_ThirdPersonCharacter` (`GameplayStatics.GetPlayerCharacter` 0)))
      (if (not (`NavMovementInterface.IsFalling` (`Character.CharacterMovement` _asbp_third_person_character)))
        (bind (_bblockinghit _binitialoverlap _time _distance _location _impactpoint _normal _impactnormal _physmat _hitactor) (`GameplayStatics.BreakHitResult` _outhit))
        (if (!= _possesableobject _hitactor)
          (`/Engine/EditorBlueprintResources/StandardMacros.IsValid` _possesableobject
            (:`Is Valid`
              (`MeshComponent.SetOverlayMaterial` (`self.GetComponentByClass` (`self.PossesableObject`) "/Script/Engine.StaticMeshComponent") "/Game/LEVEL/Pigeon/BirdBronze/BirdBronze_Material.BirdBronze_Material"))
            (:`Is Not Valid`
              _)))
        (`/Engine/EditorBlueprintResources/StandardMacros.IsValid` (`self.GetComponentByClass` _hitactor "/Game/LEVEL/Possess.Possess_C")
          (:`Is Valid`
            (set `self.isSeeingtheObject` true)
            (`MeshComponent.SetOverlayMaterial` (`self.GetComponentByClass` _hitactor "/Script/Engine.StaticMeshComponent") "/Game/LEVEL/Pigeon/OutlineMaterial.OutlineMaterial")
            (set `self.PossesableObject` _hitactor))
          (:`Is Not Valid`
            (set `self.isSeeingtheObject` false))))
      (elif (`self.isSeeingtheObject`)
        (set `self.isSeeingtheObject` false)
        (`MeshComponent.SetOverlayMaterial` (`self.GetComponentByClass` (`self.PossesableObject`) "/Script/Engine.StaticMeshComponent") "/Game/LEVEL/Pigeon/BirdBronze/BirdBronze_Material.BirdBronze_Material")))))

(event `EnhancedInput|/Game/LEVEL/IA_Possess`
  (params (ActionValue :type Boolean) (ElapsedSeconds :type "Float (double-precision)") (TriggeredSeconds :type "Float (double-precision)") (InputAction :type "InputAction Object Reference" :default "/Game/LEVEL/IA_Possess.IA_Possess"))
  (bind _returnvalue (`GameplayStatics.GetPlayerCharacter` 0))
  (bind _possesableobject (`self.PossesableObject`))
  (:`Triggered`
    (bind _asbp_main_game_instance (cast `/Game/InteractiveInventory/Blueprints/GameModes-Inventory/BP_MainGameInstance` (`GameplayStatics.GetGameInstance`)))
    (if (`/Game/InteractiveInventory/Blueprints/GameModes-Inventory/BP_MainGameInstance.BirdCollisionBool` _asbp_main_game_instance)
      (if (`self.isSeeingtheObject`)
        (bind _asbp_third_person_character (cast `/Game/InteractiveInventory/Blueprints/GameModes-Inventory/BP_ThirdPersonCharacter` _returnvalue))
        (`self.DisableInput` null)
        (if (not (`NavMovementInterface.IsFalling` (`Character.CharacterMovement` _asbp_third_person_character)))
          (bind _asbp_third_person_character_2 (cast `/Game/InteractiveInventory/Blueprints/GameModes-Inventory/BP_ThirdPersonCharacter` _returnvalue))
          (`ActorComponent.Deactivate` (`Character.CharacterMovement` _asbp_third_person_character_2))
          (bind _returnvalue_2 (`NiagaraFunctionLibrary.SpawnSystemAtLocation` "/Game/LEVEL/NiagaraVFX/Circle/CircleNiagara.CircleNiagara" (`SceneComponent.GetSocketLocation` (`Character.Mesh` _asbp_third_person_character) "foot_l") (struct) (1.0 1.0 1.0) false :!label _label))
          (`/Game/InteractiveInventory/Blueprints/GameModes-Inventory/BP_ThirdPersonCharacter.MagicCircle` _asbp_third_person_character_2 false)
          (bind _output_get (set `self.CircleAnimation` _returnvalue_2))
          (`/Engine/EditorBlueprintResources/StandardMacros.IsValid` _output_get
            (:`Is Valid`
              (`Character.PlayAnimMontage` _asbp_third_person_character_2 "/Game/GameMap/Hermes/HermesAnimations/AS_P_Aim_01_Montage.AS_P_Aim_01_Montage" 0.1 "None")
              (set `SkeletalMeshComponent.GlobalAnimRateScale` 1.0 (`Character.Mesh` _asbp_third_person_character_2))
              (`KismetSystemLibrary.Delay` 0.8)
              (`self.UnPossess`)
              (bind _aspossesable_bird (cast `/Game/LEVEL/Possesable_Bird` _possesableobject))
              (bind _staticmesh (`/Game/LEVEL/Possesable_Bird.StaticMesh` _aspossesable_bird))
              (`StaticMeshComponent.SetStaticMesh` _staticmesh "/Game/LEVEL/Pigeon/Bird/lowbird.lowbird")
              (`PrimitiveComponent.SetMaterial` _staticmesh 0 "/Game/LEVEL/Pigeon/Bird/Bird_Material.Bird_Material")
              (bind _aspawn (cast `Pawn` _possesableobject))
              (`self.Possess` _aspawn)
              (`/Game/LEVEL/Possess.ActivatePossess` (`self.GetComponentByClass` _possesableobject "/Game/LEVEL/Possess.Possess_C"))
              (set `self.Isbirdpossesed` true)
              (`self.EnableInput` null))
            (:`Is Not Valid`
              (goto _label))))))))

(event `EnhancedInput|/Game/LEVEL/IA_Return`
  (params (ActionValue :type Boolean) (ElapsedSeconds :type "Float (double-precision)") (TriggeredSeconds :type "Float (double-precision)") (InputAction :type "InputAction Object Reference" :default "/Game/LEVEL/IA_Return.IA_Return"))
  (bind _circleanimation (`self.CircleAnimation`))
  (:`Triggered`
    (if (!= (`self.K2_GetPawn`) (`self.StartingControl`))
      (`KismetSystemLibrary.PrintText` "Hello")
      (bind _aspawn (cast `Pawn` (`GameplayStatics.GetPlayerPawn` 0)))
      (if (not (`NavMovementInterface.IsFalling` (`Pawn.GetMovementComponent` _aspawn)))
        (`PlayerCameraManager.StartCameraFade` :`self` (`PlayerController.PlayerCameraManager` (`GameplayStatics.GetPlayerController` 0)) :`FromAlpha` 1.0 :`Duration` 1.0)
        (bind _aspossesable_bird (cast `/Game/LEVEL/Possesable_Bird` (`self.PossesableObject`)))
        (bind _staticmesh (`/Game/LEVEL/Possesable_Bird.StaticMesh` _aspossesable_bird))
        (`StaticMeshComponent.SetStaticMesh` _staticmesh "/Game/LEVEL/Pigeon/BirdBronze/lowbirdbronze.lowbirdbronze")
        (`PrimitiveComponent.SetMaterial` _staticmesh 0 "/Game/LEVEL/Pigeon/BirdBronze/BirdBronze_Material.BirdBronze_Material")
        (`self.UnPossess`)
        (`/Game/LEVEL/Possess.DeactivatePossess` (`self.GetComponentByClass` (`self.PossesableObject`) "/Game/LEVEL/Possess.Possess_C"))
        (`self.Possess` (`self.StartingControl`))
        (bind _asbp_third_person_character (cast `/Game/InteractiveInventory/Blueprints/GameModes-Inventory/BP_ThirdPersonCharacter` (`GameplayStatics.GetPlayerCharacter` 0)))
        (bind _aspossesable_bird_2 (cast `/Game/LEVEL/Possesable_Bird` (`self.PossesableObject`)))
        (`self.K2_SetActorLocationAndRotation` _aspossesable_bird_2 (`/Game/LEVEL/Possesable_Bird.DefaultLocation` _aspossesable_bird_2) (`/Game/LEVEL/Possesable_Bird.DefaultRotator` _aspossesable_bird_2) false false)
        (`/Game/InteractiveInventory/Blueprints/GameModes-Inventory/BP_ThirdPersonCharacter.MagicCircle` _asbp_third_person_character true)
        (`ActorComponent.SetComponentTickEnabled` _circleanimation false)
        (`ActorComponent.K2_DestroyComponent` _circleanimation)
        (`ActorComponent.Activate` (`Character.CharacterMovement` _asbp_third_person_character) false)
        (`Character.StopAnimMontage` _asbp_third_person_character "/Game/GameMap/Hermes/HermesAnimations/AS_P_Aim_01_Montage.AS_P_Aim_01_Montage")))))

(event `Key|G`
  (params (Key :type "Key Structure")))

(fn `EnableUI_Input`
  (params (Enable :type Boolean))
  ;[1 1 1] Set the input mode to UI
  (if Enable
    (set `self.bShowMouseCursor` true)
    (`WidgetBlueprintLibrary.SetInputMode_UIOnlyEx` self null "DoNotLock" true)
    (else
      (set `self.bShowMouseCursor` false)
      (`WidgetBlueprintLibrary.SetInputMode_GameOnly` self))))

(fn `UserConstructionScript`)