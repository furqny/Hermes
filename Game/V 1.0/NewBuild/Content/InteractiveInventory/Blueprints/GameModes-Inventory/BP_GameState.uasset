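; Game state for the interactive inventory game that creates the shared managers and runs the in-game clock.
; On BeginPlay the authority spawns the storage, shop and typewriter manager actors and keeps references to them.
; Tick, which has no authority check, advances a scaled 24-hour time, increments the day on wrap and calls OnHourChanged whenever the whole hour changes.
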(event `self.ReceiveBeginPlay`
  (`/Engine/EditorBlueprintResources/ActorMacros.Switch Has Authority`
    (:`Authority`
      (`|ExecutionSequence`
        (:`then_0`
          (bind _returnvalue (`|SpawnActorFromClass` "/Game/InteractiveInventory/Blueprints/Inventory/Storage/BP_StorageManagerActor.BP_StorageManagerActor_C" (`KismetMathLibrary.MakeTransform` (0.0 0.0 0.0)) "Undefined" "MultiplyWithRoot" null null))
          (set `self.StorageManagerRef` _returnvalue))
        (:`then_1`
          (bind _returnvalue_2 (`|SpawnActorFromClass` "/Game/InteractiveInventory/Blueprints/Inventory/Shop/BP_ShopManagerActor.BP_ShopManagerActor_C" (`KismetMathLibrary.MakeTransform` (0.0 0.0 0.0)) "Undefined" "MultiplyWithRoot" null null))
          (set `self.ShopManagerRef` _returnvalue_2))
        (:`then_2`
          (bind _returnvalue_3 (`|SpawnActorFromClass` "/Game/InteractiveInventory/Blueprints/Saves/BP_TypewriterManagerActor.BP_TypewriterManagerActor_C" (`KismetMathLibrary.MakeTransform` (0.0 0.0 0.0)) "Undefined" "MultiplyWithRoot" null null))
          (set `self.TypewriterManagerRef` _returnvalue_3))))))

(event `self.ReceiveTick`
  (params (DeltaSeconds :type "Float (single-precision)"))
  (bind _returnvalue (`KismetMathLibrary.FTrunc` (`self.CurrentTime`)))
  (bind _output_get (set `self.CurrentTime` (+ (* DeltaSeconds (`self.TimeMultiplier`)) (`self.CurrentTime`))))
  (if (>= _output_get 24.0)
    (set `self.CurrentTime` (- _output_get 24.0))
    (set `self.CurrentDay` (+ (`self.CurrentDay`) 1)))
  (if (!= _returnvalue (`self.LastRecordedHour`))
    (`self.OnHourChanged` _returnvalue)
    (set `self.LastRecordedHour` _returnvalue)))

(fn `UserConstructionScript`)