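; BP_HermesButton is a pressure button that tracks whether Hermes, detected as any BP_ThirdPersonCharacter, is standing on it.
; Begin and end overlaps on its Collision component update a boolean, with a guard against repeated presses on entry only.
; Each change prints a Turkish debug message and broadcasts the state through the HermesButtonPressed dispatcher.
; Overlapping characters are not counted, so any exit releases the button.
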(event `self.Collision.OnComponentBeginOverlap`
  (params (OverlappedComponent :type "PrimitiveComponent Object Reference") (OtherActor :type "Actor Object Reference") (OtherComp :type "PrimitiveComponent Object Reference") (OtherBodyIndex :type Integer) (bFromSweep :type Boolean) (SweepResult :type "HitResult Structure (by ref)"))
  (cast `/Game/InteractiveInventory/Blueprints/GameModes-Inventory/BP_ThirdPersonCharacter` OtherActor)
  (if (not (`self.Ishermesonthebutton`))
    (bind _output_get (set `self.Ishermesonthebutton` true))
    (`KismetSystemLibrary.PrintText` "Hermes Bastı")
    (`self.HermesButtonPressed` _output_get)))

(event `self.Collision.OnComponentEndOverlap`
  (params (OverlappedComponent :type "PrimitiveComponent Object Reference") (OtherActor :type "Actor Object Reference") (OtherComp :type "PrimitiveComponent Object Reference") (OtherBodyIndex :type Integer))
  (cast `/Game/InteractiveInventory/Blueprints/GameModes-Inventory/BP_ThirdPersonCharacter` OtherActor)
  (bind _output_get (set `self.Ishermesonthebutton` false))
  (`KismetSystemLibrary.PrintText` "Hermes  Basmadı!")
  (`self.HermesButtonPressed` _output_get))

(fn `UserConstructionScript`)