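; BP_PlatformandDance is a dance puzzle platform that locks the player in place on overlap and enables dancing until the sequence is solved or failed.
; DanceCount checks each dance input against CorrectOrder, advancing on a match and counting mistakes otherwise.
; Success plays a sound, restores walking and, after a delay, opens Symbolsphere.
; Too many mistakes trigger a camera fade, teleport the player to DanceRespawn and reset the puzzle.
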(event `self.Collision.OnComponentBeginOverlap`
  (params (OverlappedComponent :type "PrimitiveComponent Object Reference") (OtherActor :type "Actor Object Reference") (OtherComp :type "PrimitiveComponent Object Reference") (OtherBodyIndex :type Integer) (bFromSweep :type Boolean) (SweepResult :type "HitResult Structure (by ref)"))
  (bind _asbp_third_person_character (cast `/Game/InteractiveInventory/Blueprints/GameModes-Inventory/BP_ThirdPersonCharacter` OtherActor))
  (if (`self.Puzzlefinished`)
    _
    (elif (not (`self.Bpuzzleactive`))
      (set `self.Bpuzzleactive` true)
      (set `/Game/InteractiveInventory/Blueprints/GameModes-Inventory/BP_ThirdPersonCharacter.Bcandance` true _asbp_third_person_character)
      (set `/Game/InteractiveInventory/Blueprints/GameModes-Inventory/BP_ThirdPersonCharacter.PlatformandDance` self _asbp_third_person_character)
      (`CharacterMovementComponent.DisableMovement` (`Character.CharacterMovement` _asbp_third_person_character)))))

(event `self.Collision.OnComponentEndOverlap`
  (params (OverlappedComponent :type "PrimitiveComponent Object Reference") (OtherActor :type "Actor Object Reference") (OtherComp :type "PrimitiveComponent Object Reference") (OtherBodyIndex :type Integer))
  (bind _asbp_third_person_character (cast `/Game/InteractiveInventory/Blueprints/GameModes-Inventory/BP_ThirdPersonCharacter` OtherActor))
  (set `/Game/InteractiveInventory/Blueprints/GameModes-Inventory/BP_ThirdPersonCharacter.Bcandance` false _asbp_third_person_character)
  (set `/Game/InteractiveInventory/Blueprints/GameModes-Inventory/BP_ThirdPersonCharacter.PlatformandDance` null _asbp_third_person_character))

(event `DanceCount`
  (params (Input :type Integer))
  (if (`self.Bpuzzleactive`)
    (if (== Input (`|GetArrayItem` (`self.CorrectOrder`) (`self.Currentindex`)))
      (`KismetArrayLibrary.Array_Add` (`self.PlayerOrder`) Input)
      (`/Engine/EditorBlueprintResources/StandardMacros.IncrementInt` (`self.Currentindex`)
        (:`  `
          (if (>= (`self.Currentindex`) (`KismetArrayLibrary.Array_Length` (`self.CorrectOrder`)))
            (`KismetSystemLibrary.PrintString` "Puzzle Succesed!")
            (`self.PuzzleSuccess`)
            (else
              (`KismetSystemLibrary.PrintString` "Not Yet!")))))
      (else
        (`KismetSystemLibrary.PrintText` "yanlis basladin gulum")
        (`/Engine/EditorBlueprintResources/StandardMacros.IncrementInt` (`self.MistakeCount`)
          (:`  `
            (if (>= (`self.MistakeCount`) (`self.Maxmistake`))
              (`KismetSystemLibrary.PrintString` "Puzzle Fail!")
              (`self.PuzzleFail`)
              (set `self.Bpuzzleactive` false))))))))

(event `PuzzleSuccess`
  (`GameplayStatics.PlaySound2D` "/Engine/VREditor/Sounds/VR_confirm.VR_confirm" 1.0 1.0 0.0 null null)
  (bind _asbp_third_person_character (cast `/Game/InteractiveInventory/Blueprints/GameModes-Inventory/BP_ThirdPersonCharacter` (`GameplayStatics.GetPlayerCharacter` 0)))
  (set `/Game/InteractiveInventory/Blueprints/GameModes-Inventory/BP_ThirdPersonCharacter.Dialogue?` true _asbp_third_person_character)
  (set `/Game/InteractiveInventory/Blueprints/GameModes-Inventory/BP_ThirdPersonCharacter.Bcandance` false _asbp_third_person_character)
  (set `self.Bpuzzleactive` false)
  (`Character.StopJumping` _asbp_third_person_character)
  (`CharacterMovementComponent.SetMovementMode` (`Character.CharacterMovement` _asbp_third_person_character) "MOVE_Walking" 0)
  (`KismetSystemLibrary.Delay` (`/Game/InteractiveInventory/Blueprints/GameModes-Inventory/BP_ThirdPersonCharacter.Dance3duration` _asbp_third_person_character))
  (set `/Game/InteractiveInventory/Blueprints/GameModes-Inventory/BP_ThirdPersonCharacter.Dialogue?` false _asbp_third_person_character)
  (set `self.Puzzlefinished` true)
  (`/Game/LEVEL/Amphitheathre/BP_SymbolSphere.OpentheSphere` (`self.Symbolsphere`)))

(event `PuzzleFail`
  (bind _playercameramanager (`PlayerController.PlayerCameraManager` (`GameplayStatics.GetPlayerController` 0)))
  (`GameplayStatics.PlaySound2D` "/Game/sound_effects/Down1.Down1" 1.0 1.0 0.0 null null)
  (bind _asbp_third_person_character (cast `/Game/InteractiveInventory/Blueprints/GameModes-Inventory/BP_ThirdPersonCharacter` (`GameplayStatics.GetPlayerCharacter` 0)))
  (set `/Game/InteractiveInventory/Blueprints/GameModes-Inventory/BP_ThirdPersonCharacter.Bcandance` false _asbp_third_person_character)
  (`PlayerCameraManager.StartCameraFade` :`self` _playercameramanager :`ToAlpha` 1.0 :`Duration` 1.0)
  (`KismetSystemLibrary.Delay` 1.0)
  (`self.K2_SetActorLocation` _asbp_third_person_character (`/Game/LEVEL/Amphitheathre/DanceRespawn.TargetPoint` (`self.DanceRespawn`)) false false)
  (`PlayerCameraManager.StartCameraFade` :`self` _playercameramanager :`FromAlpha` 1.0 :`Duration` 1.0)
  (set `self.MistakeCount` 0)
  (set `self.Currentindex` 0)
  (`KismetArrayLibrary.Array_Clear` (`self.PlayerOrder`))
  (`CharacterMovementComponent.SetMovementMode` (`Character.CharacterMovement` _asbp_third_person_character) "MOVE_Walking" 0)
  (`Character.StopAnimMontage` _asbp_third_person_character null)
  (set `/Game/InteractiveInventory/Blueprints/GameModes-Inventory/BP_ThirdPersonCharacter.PlatformandDance` null _asbp_third_person_character))

(fn `UserConstructionScript`)