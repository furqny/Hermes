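; BP_DirectionObject is an interactable rotating object that reports whether it faces a designated correct direction, apparently as a puzzle piece.
; On InteractReceived it plays the player's pickup montage, cycles Direction through four steps and snaps the actor's yaw in quarter turns, keeping MoonRock's pitch and roll.
; It compares Direction to CorrectDirection and calls OnStateChanged only when correctness flips, using Wascorrect to track the last state.
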(event `self.InteractReceived`
  (params (NewOwner :type "Actor Object Reference"))
  (bind (_returnvalue_roll _returnvalue_pitch) (`KismetMathLibrary.BreakRotator` (`SceneComponent.K2_GetComponentRotation` (`self.MoonRock`))))
  (bind _asbp_third_person_character (cast `/Game/InteractiveInventory/Blueprints/GameModes-Inventory/BP_ThirdPersonCharacter` (`GameplayStatics.GetPlayerCharacter` 0)))
  (`Character.PlayAnimMontage` _asbp_third_person_character "/Game/GameMap/Hermes/HermesAnimations/HermesPickup.HermesPickup" 1.0 "None")
  (set `self.Direction` (+ (mod (`self.Direction`) 4) 1))
  (`self.K2_SetActorRotation` (`KismetMathLibrary.MakeRotator` _returnvalue_roll _returnvalue_pitch (`KismetMathLibrary.Lerp` (`KismetMathLibrary.Conv_IntToDouble` (* (`self.Direction`) 90)) 25.0)) true)
  (if (== (`self.CorrectDirection`) (`self.Direction`))
    (if (not (`self.wascorrect`))
      (set `self.wascorrect` true)
      (`self.OnStateChanged` true))
    (elif (`self.wascorrect`)
      (set `self.wascorrect` false)
      (`self.OnStateChanged` false))))

(fn `UserConstructionScript`)