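; Manager for a two-button co-op puzzle in which Bird and Hermes must both be on their buttons to open a gate.
; At BeginPlay it binds to both buttons' press events, and each Hermes event re-binds the Bird event until solved.
; A Bird press while Hermes is on the button sets a one-time flag and calls ButtonPuzzleGateOpen on BP_MainGameInstance.
; Debug text reports success or failure.
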(event `self.ReceiveBeginPlay`
  (add `/Game/LEVEL/BP_HermesButton.HermesButtonPressed` (`self.Bp_Hermes`) (delegate `HermesButtonPressed_Event`))
  (add `/Game/LEVEL/BP_BirdButton.BirdButtonPressed` (`self.Bp_Bird`) (delegate `BirdButtonPressed_Event`) :!label _label))

(event `BirdButtonPressed_Event`
  (params (IsBirdButtonPressed :type Boolean))
  (if (and (stale `HermesButtonPressed_Event` IsHermesOnButton) IsBirdButtonPressed)
    (if (not (`self.Diditwork`))
      (`KismetSystemLibrary.PrintText` "It worked!")
      (set `self.Diditwork` true)
      (bind _asbp_main_game_instance (cast `/Game/InteractiveInventory/Blueprints/GameModes-Inventory/BP_MainGameInstance` (`GameplayStatics.GetGameInstance`)))
      (`/Game/InteractiveInventory/Blueprints/GameModes-Inventory/BP_MainGameInstance.ButtonPuzzleGateOpen` _asbp_main_game_instance))
    (else
      (`KismetSystemLibrary.PrintText` "It didn't"))))

(event `HermesButtonPressed_Event`
  (params (IsHermesOnButton :type Boolean))
  (if (not (`self.Diditwork`))
    (goto _label)))

(fn `UserConstructionScript`)