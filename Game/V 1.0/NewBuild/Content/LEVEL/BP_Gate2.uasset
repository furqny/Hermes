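; BP_Gate2 is a gate that moves vertically when the game instance's ButtonPuzzleSolved event fires.
; On that event it sets CinematicInterrupt on the player controller and plays the S_ButtonSolved level sequence.
; When the sequence finishes, a timeline drives the static mesh's world Z as an absolute height, keeping X and Y.
; CinematicInterrupt is cleared from the timeline's Update, so it resets as the movement starts.
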(event `self.ReceiveBeginPlay`
  (bind _asbp_main_game_instance (cast `/Game/InteractiveInventory/Blueprints/GameModes-Inventory/BP_MainGameInstance` (`GameplayStatics.GetGameInstance`)))
  (add `/Game/InteractiveInventory/Blueprints/GameModes-Inventory/BP_MainGameInstance.ButtonPuzzleSolved` _asbp_main_game_instance (delegate `RaiseGate`)))

(event `RaiseGate`
  (bind _asbp_player_controller (cast `/Game/InteractiveInventory/Blueprints/GameModes-Inventory/BP_PlayerController` (`GameplayStatics.GetPlayerController` 0)))
  (set `/Game/InteractiveInventory/Blueprints/GameModes-Inventory/BP_PlayerController.CinematicInterrupt` true _asbp_player_controller)
  (bind (_outactor _returnvalue) (`LevelSequencePlayer.CreateLevelSequencePlayer` "/Game/LEVEL/S_ButtonSolved.S_ButtonSolved"))
  (`MovieSceneSequencePlayer.Play` _returnvalue)
  (add `MovieSceneSequencePlayer.OnFinished` _returnvalue (delegate `Finished`)))

(event `Finished`
  (bind _staticmesh (`self.StaticMesh`))
  (bind (_returnvalue_x _returnvalue_y) (`KismetMathLibrary.BreakVector` (`SceneComponent.K2_GetComponentLocation` _staticmesh)))
  (bind (_direction _newtrack_0) (`Timeline|Zaman Çizelgesi`)
    (:`Update`
      (`SceneComponent.K2_SetWorldLocation` _staticmesh (`KismetMathLibrary.MakeVector` _returnvalue_x _returnvalue_y _newtrack_0) false false)
      (set `/Game/InteractiveInventory/Blueprints/GameModes-Inventory/BP_PlayerController.CinematicInterrupt` false (stale `RaiseGate` _asbp_player_controller)))))

(fn `UserConstructionScript`)