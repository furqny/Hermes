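; A pressure button for the possessable bird that reports its state through a BirdButtonPressed call.
; Overlap plays a sound and a timeline that moves the button on Z; if the bird is still on it at the end, it reports pressed and latches permanently via GateDone.
; Any pawn leaving before then reverses the timeline and reports unpressed.
; When the game instance's Birddontfly flag is set, pressing also freezes the bird's movement and flight temporarily.
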(event `self.Collision.OnComponentBeginOverlap`
  (params (OverlappedComponent :type "PrimitiveComponent Object Reference") (OtherActor :type "Actor Object Reference") (OtherComp :type "PrimitiveComponent Object Reference") (OtherBodyIndex :type Integer) (bFromSweep :type Boolean) (SweepResult :type "HitResult Structure (by ref)"))
  (bind _bird_button1 (`self.Bird_Button1`))
  (bind (_relativelocation_x _relativelocation_y) (`KismetMathLibrary.BreakVector` (`SceneComponent.RelativeLocation` _bird_button1)))
  (bind _aspawn (cast `Pawn` OtherActor))
  (bind _aspossesable_bird (cast `/Game/LEVEL/Possesable_Bird` _aspawn))
  (set `self.Birdon` true)
  (if (not (`self.GateDone`))
    (`GameplayStatics.PlaySound2D` "/Game/sound_effects/button.button" 1.0 1.0 0.0 null null)
    (bind (_direction _newtrack_0) (`Timeline|Zaman Çizelgesi` :!via `PlayFromStart` :!label _label)
      (:`Update`
        (`SceneComponent.K2_SetRelativeLocation` _bird_button1 (`KismetMathLibrary.MakeVector` _relativelocation_x _relativelocation_y _newtrack_0) false false))
      (:`Finished`
        (if (`self.Birdon`)
          (`KismetSystemLibrary.PrintText` "Kuş Bastı!")
          (`self.BirdButtonPressed` true)
          (set `self.GateDone` true)
          (bind _asbp_main_game_instance (cast `/Game/InteractiveInventory/Blueprints/GameModes-Inventory/BP_MainGameInstance` (`GameplayStatics.GetGameInstance`)))
          (if (`/Game/InteractiveInventory/Blueprints/GameModes-Inventory/BP_MainGameInstance.Birddontfly` _asbp_main_game_instance)
            (bind _charactermovement (`Character.CharacterMovement` _aspossesable_bird))
            (`CharacterMovementComponent.DisableMovement` _charactermovement)
            (set `/Game/LEVEL/Possesable_Bird.NoFly` true _aspossesable_bird)
            (`KismetSystemLibrary.Delay` 7.0)
            (`CharacterMovementComponent.SetMovementMode` _charactermovement "MOVE_Walking" 0)
            (set `/Game/LEVEL/Possesable_Bird.NoFly` false _aspossesable_bird)))))))

(event `self.Collision.OnComponentEndOverlap`
  (params (OverlappedComponent :type "PrimitiveComponent Object Reference") (OtherActor :type "Actor Object Reference") (OtherComp :type "PrimitiveComponent Object Reference") (OtherBodyIndex :type Integer))
  (cast `Pawn` OtherActor)
  (set `self.Birdon` false)
  (if (not (`self.GateDone`))
    (`|ExecutionSequence`
      (:`then_0`
        (goto _label :!via `ReverseFromEnd`))
      (:`then_1`
        (bind _output_get (set `self.Isbirdonthebutton` false))
        (`KismetSystemLibrary.PrintText` "Kuş Basmadı!")
        (`self.BirdButtonPressed` _output_get)))))

(fn `UserConstructionScript`)