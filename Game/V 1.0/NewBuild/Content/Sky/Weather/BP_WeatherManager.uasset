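; BP_WeatherManager darkens the level's sun as the player's karma drops into negative bands.
; On BeginPlay it tints the first DirectionalLight found and binds to the game instance's karma-changed event.
; A timeline lerps intensity to each band's target, while color snaps and MPC_Weather Wetness is set to zero.
; Karma from -100 up to below -20, or non-negative, triggers no change, so the sun never brightens back at zero.
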(event `self.ReceiveBeginPlay`
  (bind _asbp_main_game_instance (cast `/Game/InteractiveInventory/Blueprints/GameModes-Inventory/BP_MainGameInstance` (`GameplayStatics.GetGameInstance`)))
  (bind _outactors (`GameplayStatics.GetAllActorsOfClass` "/Script/Engine.DirectionalLight"))
  (bind _output_get (set `self.SunLight` (`|GetArrayItem` _outactors)))
  (`LightComponent.SetLightColor` (`Light.LightComponent` _output_get) (struct :`R` 0.522493 :`G` 0.997135 :`B` 1.0 :`A` 1.0) true)
  (add `/Game/InteractiveInventory/Blueprints/GameModes-Inventory/BP_MainGameInstance.OnKarmaChanged` _asbp_main_game_instance (delegate `OnKarmaChanged_Event`)))

(event `OnKarmaChanged_Event`
  (params (CurrentKarma :type Integer))
  (`|ExecutionSequence`
    (:`then_0`
      (if (< CurrentKarma 0)
        (if (>= CurrentKarma -5)
          (`self.SetDarkWeather` 18.0 (struct :`R` 0.194618 :`G` 0.617207 :`B` 0.679543 :`A` 1.0)))))
    (:`then_1`
      (if (< CurrentKarma -5)
        (if (>= CurrentKarma -10)
          (`self.SetDarkWeather` 16.0 (struct :`R` 0.104634 :`G` 0.247534 :`B` 0.395833 :`A` 1.0))
          (`KismetSystemLibrary.PrintString` "STORMY WEATHER" true true (struct :`R` 1.0 :`G` 0.035426 :`B` 0.846088 :`A` 1.0) 5.0))))
    (:`then_2`
      (if (< CurrentKarma -10)
        (if (>= CurrentKarma -20)
          (`self.SetDarkWeather` 14.0 (struct :`R` 0.042234 :`G` 0.060234 :`B` 0.255208 :`A` 1.0))
          (`KismetSystemLibrary.PrintString` "HOHOHOOHO" true true (struct :`R` 1.0 :`G` 0.035426 :`B` 0.846088 :`A` 1.0) 5.0))))
    (:`then_3`
      (if (< CurrentKarma -100)
        (`self.SetDarkWeather` 3.0 (struct :`R` 0.007916 :`G` 0.009492 :`B` 0.078125 :`A` 1.0))
        (`KismetSystemLibrary.PrintString` "HOHOHOOHO" true true (struct :`R` 1.0 :`G` 0.035426 :`B` 0.846088 :`A` 1.0) 5.0)))))

(event `SetDarkWeather`
  (params (Intensity :type "Float (double-precision)") (NewParam :type "LinearColor Structure"))
  (bind _lightcomponent (`Light.LightComponent` (`self.SunLight`)))
  (set `self.TargetIntensity` Intensity)
  (set `self.StartIntensity` (`LightComponentBase.Intensity` (`Light.LightComponent` (`self.SunLight`))))
  (bind (_direction _alpha) (`Timeline|WeatherTransition` :!via `PlayFromStart`)
    (:`Update`
      (`LightComponent.SetIntensity` _lightcomponent (`KismetMathLibrary.Lerp` (`self.StartIntensity`) (`self.TargetIntensity`) _alpha))
      (`LightComponent.SetLightColor` _lightcomponent NewParam true)
      (`KismetMaterialLibrary.SetScalarParameterValue` "/Game/Sky/Weather/MPC_Weather.MPC_Weather" "Wetness"))))

(fn `UserConstructionScript`)